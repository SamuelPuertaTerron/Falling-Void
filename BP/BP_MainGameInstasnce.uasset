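; Game instance for a two-player wave-combat game, holding difficulty tuning, main HUD creation, samurai respawn-and-possess, and slow-motion win/lose screens.
; Difficulty tiers set damage, health and speed values; SetEnemyDiffculty copies health and damage onto enemies.
; Loss triggers when both Robot and Samurai are down.
; The deprecated wave spawner retains capped, alternating-side melee and spitter spawns, but its StartWave and WaveManager events are empty, leaving wave progression disconnected.
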(event Custom|Start%20Wave
  (params (Melees :type Integer) (Spitters :type Integer))
  ;[1 0 0] Deprecated. A new system has been created
)

(event Custom|Spawn%20Spitter
  ;[1 0 0] Deprecated. A new system has been created
  (Math|Integer|IncrementInt (Variables|Default|GetSpitters%20Spawned)
    (:%20%20
      (Utilities|FlowControl|FlipFlop
        (:A
          (AI|SpawnAIFromClass "/Game/BP/Enemy/BP_SpitterEnemy.BP_SpitterEnemy_C" "/Game/BP/Enemy/AI/BT_MeleeEnemy.BT_MeleeEnemy" (Math|Vector|MakeVector (Variables|Default|GetLocation%20X%202) -3.8e+03 4.8e+02) "0, 0, 0" true 0)
          (bind _output_get (Variables|Default|SetLocation%20X%202 (+ (Variables|Default|GetLocation%20X%202) 1e+02)))
          (if (>= _output_get 5.7e+03)
            (Variables|Default|SetLocation%20X%202 4.7e+03)))
        (:B
          (AI|SpawnAIFromClass "/Game/BP/Enemy/BP_SpitterEnemy.BP_SpitterEnemy_C" "/Game/BP/Enemy/AI/BT_MeleeEnemy.BT_MeleeEnemy" (Math|Vector|MakeVector (Variables|Default|GetLocation%20X%201) -9.05e+03 3.3e+02) "0, 0, 0" true 0)
          (bind _output_get_2 (Variables|Default|SetLocation%20X%201 (+ (Variables|Default|GetLocation%20X%201) 1e+02)))
          (if (>= _output_get_2 5.7e+03)
            (Variables|Default|SetLocation%20X%201 4.7e+03)))))))

(event Custom|Spawn%20Melee
  ;[1 0 0] Deprecated. A new system has been created
  (Math|Integer|IncrementInt (Variables|Default|GetMelees%20Spawned)
    (:%20%20
      (Utilities|FlowControl|FlipFlop
        (:A
          (AI|SpawnAIFromClass "/Game/BP/Enemy/BP_MeleeWorking.BP_MeleeWorking_C" "/Game/BP/Enemy/AI/BT_MeleeEnemy.BT_MeleeEnemy" (Math|Vector|MakeVector (Variables|Default|GetLocation%20X%201) -9.05e+03 3.3e+02) "0, 0, 0" true 0)
          (bind _output_get (Variables|Default|SetLocation%20X%201 (+ (Variables|Default|GetLocation%20X%201) 1e+02)))
          (if (>= _output_get 5.7e+03)
            (Variables|Default|SetLocation%20X%201 4.7e+03)))
        (:B
          (AI|SpawnAIFromClass "/Game/BP/Enemy/BP_MeleeWorking.BP_MeleeWorking_C" "/Game/BP/Enemy/AI/BT_MeleeEnemy.BT_MeleeEnemy" (Math|Vector|MakeVector (Variables|Default|GetLocation%20X%202) -3.9e+03 4.8e+02) "0, 0, 0" true 0)
          (bind _output_get_2 (Variables|Default|SetLocation%20X%202 (+ (Variables|Default|GetLocation%20X%202) 1e+02)))
          (if (>= _output_get_2 5.7e+03)
            (Variables|Default|SetLocation%20X%202 4.7e+03)))))))

(event Custom|Melees
  ;[1 0 0] Deprecated. A new system has been created
  (if (< (- (Variables|Default|GetMelees%20Spawned) (Variables|Default|GetMelees%20Killed)) 10)
    (CallFunction|SpawnMelee)
    (CallFunction|WaveManager)))

(event Custom|Spitters
  ;[1 0 0] Deprecated. A new system has been created
  (if (< (- (Variables|Default|GetSpitters%20Spawned) (Variables|Default|GetSpitters%20Killed)) 2)
    (CallFunction|SpawnSpitter)
    (CallFunction|WaveManager)))

(event Custom|Add%20UI
  (bind _returnvalue (Game|GetPlayerController 0))
  (bind _returnvalue_2 (UserInterface|CreateWidget "/Game/UMG/UMG_Main.UMG_Main_C" _returnvalue))
  (bind _output_get (Variables|Default|SetUI _returnvalue_2))
  (UserInterface|Viewport|AddtoViewport _output_get 0)
  (Input|SetInputModeGameOnly _returnvalue false)
  (Variables|/Script/Engine.PlayerController|SetbShowMouseCursor _returnvalue false))

(event Custom|Spawn%20Enemies
  ;[1 0 0] Deprecated. A new system has been created
  (Utilities|FlowControl|Sequence
    (:then_0
      (if (!= (Variables|Default|GetMelees%20To%20Spawn) (Variables|Default|GetMelees%20Spawned))
        (CallFunction|Melees)))
    (:then_1
      (if (!= (Variables|Default|GetSpitters%20To%20Spawn) (Variables|Default|GetSpitters%20Spawned))
        (CallFunction|Spitters)))))

(event Custom|Wave%20Info
  (params (Melees :type Integer) (Spitters :type Integer))
  ;[1 0 0] Deprecated. A new system has been created
  (if (== (Variables|Default|GetEnemies%20killed) (Variables|Default|GetEnemies%20to%20Spawn))
    (if (Variables|Default|GetWave%20Preped)
      (CallFunction|ResetSpawns)
      (Utilities|FlowControl|Delay 3.0)
      (CallFunction|StartWave Melees Spitters)
      (else
        (Math|Integer|IncrementInt (Variables|Default|GetWave)
          (:%20%20
            (Variables|Default|SetWave%20Preped true)
            (CallFunction|WaveManager)))))
    (else
      (CallFunction|SpawnEnemies))))

(event Custom|Wave%200
  ;[1 0 0] Deprecated. A new system has been created
)

(event Custom|Winning
  (bind _returnvalue (Game|GetPlayerController 0))
  (bind _ui (Variables|Default|GetUI))
  (bind _umg_level1complete (Variables|/Game/UMG/UMG_Main.UMG_Main_C|GetUMG_Level1Complete _ui))
  (Variables|Default|SetRobot%20Down? false)
  (Variables|Default|SetSamurai%20Down? false)
  (Utilities|Time|SetGlobalTimeDilation 0.1)
  (Widget|SetVisibility _umg_level1complete "Visible")
  (UserInterface|Animation|PlayAnimation _umg_level1complete (Variables|/Game/UMG/UMG_Level1Complete.UMG_Level1Complete_C|GetBlackoutFade _umg_level1complete) 0.0 1 "Forward" 1.0 false)
  (Utilities|FlowControl|Delay 0.5)
  (Widget|SetVisibility (Variables|/Game/UMG/UMG_Level1Complete.UMG_Level1Complete_C|GetLoserBorder _umg_level1complete) "Visible")
  (Utilities|Time|SetGlobalTimeDilation 1.0)
  (Input|SetInputModeGameandUI _returnvalue _umg_level1complete "DoNotLock" true false)
  (Variables|/Script/Engine.PlayerController|SetbShowMouseCursor _returnvalue true)
  (Input|SetInputModeGameandUI (Game|GetPlayerController 1) _umg_level1complete "DoNotLock" true false))

(event Custom|Diffculty%20Mods
  (switch int (Variables|Default|GetDiffculty)
    (:1
      (Variables|Default|SetEnemy%20Dmg%20Boost 0.8)
      (Variables|Default|SetEnemy%20Health 1e+02)
      (Variables|Default|SetEnemy%20speed 6e+02))
    (:2
      (Variables|Default|SetEnemy%20Dmg%20Boost 1.0)
      (Variables|Default|SetEnemy%20Health 2e+02)
      (Variables|Default|SetEnemy%20speed 6e+02))
    (:3
      (Variables|Default|SetEnemy%20Dmg%20Boost 1.2)
      (Variables|Default|SetEnemy%20Health 4e+02)
      (Variables|Default|SetEnemy%20speed 6e+02))
    (:4
      (Variables|Default|SetEnemy%20Dmg%20Boost 5.0)
      (Variables|Default|SetEnemy%20Health 1e+03)
      (Variables|Default|SetEnemy%20speed 8.5e+02))))

(event Custom|SwapCharacter
  (params (Transform :type Transform) (Target :type Actor%20Object%20Reference))
  (bind _output_get (Variables|Default|SetTransform Transform))
  (Actor|DestroyActor Target)
  (bind _returnvalue (Game|SpawnActorfromClass "/Game/BP/BP_PlayerSamurai.BP_PlayerSamurai_C" _output_get "Undefined" "MultiplyWithRoot" 0 0))
  (Pawn|Possess (Game|GetPlayerController (Variables|Default|GetPlayer%20To%20Swap)) _returnvalue)
  (Variables|/Game/BP/BP_PlayerSamurai.BP_PlayerSamurai_C|SetMGI _returnvalue self))

(event Custom|Check%20for%20losing
  (bind _returnvalue (Game|GetPlayerController 0))
  (bind _ui (Variables|Default|GetUI))
  (bind _umg_gameover (Variables|/Game/UMG/UMG_Main.UMG_Main_C|GetUMG_GameOver _ui))
  (if (and (Variables|Default|GetRobot%20Down?) (Variables|Default|GetSamurai%20Down?))
    (Variables|Default|SetRobot%20Down? false)
    (Variables|Default|SetSamurai%20Down? false)
    (Utilities|Time|SetGlobalTimeDilation 0.1)
    (Widget|SetVisibility _umg_gameover "Visible")
    (UserInterface|Animation|PlayAnimation _umg_gameover (Variables|/Game/UMG/UMG_GameOver.UMG_GameOver_C|GetBlackoutFade _umg_gameover) 0.0 1 "Forward" 1.0 false)
    (Utilities|FlowControl|Delay 0.5)
    (Widget|SetVisibility (Variables|/Game/UMG/UMG_GameOver.UMG_GameOver_C|GetLoserBorder _umg_gameover) "Visible")
    (Utilities|Time|SetGlobalTimeDilation 1.0)
    (Input|SetInputModeGameandUI _returnvalue _umg_gameover "DoNotLock" true false)
    (Variables|/Script/Engine.PlayerController|SetbShowMouseCursor _returnvalue true)
    (Input|SetInputModeGameandUI (Game|GetPlayerController 1) _umg_gameover "DoNotLock" true false)))

(event Custom|Wave%20Manager
  ;[1 0 0] Deprecated. A new system has been created
)

(event Custom|Reset%20spawns
  ;[1 0 0] Deprecated. A new system has been created
  (Variables|Default|SetMelees%20Spawned 0)
  (Variables|Default|SetSpitters%20Spawned 0)
  (Variables|Default|SetEnemies%20killed 0)
  (Variables|Default|SetSpitters%20Killed 0)
  (Variables|Default|SetMelees%20Killed 0)
  (Variables|Default|SetWave%20Preped false))

(event EventInit)

(fn SetEnemyDiffculty
  (params (Enemy :type FV%20Enemy%20Base%20Object%20Reference))
  (bind _enemy_health (Variables|Default|GetEnemy%20Health))
  (Variables|/Script/FallingVoid.FVBaseCharacter|SetHealth Enemy _enemy_health)
  (Variables|/Script/FallingVoid.FVBaseCharacter|SetMaxHealth Enemy _enemy_health)
  (Variables|/Script/FallingVoid.FVBaseCharacter|SetDamageBoost Enemy (Variables|Default|GetEnemy%20Dmg%20Boost)))