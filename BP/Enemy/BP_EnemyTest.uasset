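; BP_EnemyTest is a test enemy that attacks on a timer and destroys itself on death.
; On BeginPlay it caches the main game instance and passes itself to SetEnemyDiffculty.
; Tick drives a one-second Delay, which ignores re-triggers while pending, so Attack fires roughly once per second.
; OnDied prints a debug message and destroys the actor; Attack's logic is not defined in this graph.
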(event EventBeginPlay
  (bind _asbp_main_game_instasnce (Utilities|Casting|CastToBP_MainGameInstasnce (Game|GetGameInstance)))
  (bind _output_get (Variables|Default|SetMGI _asbp_main_game_instasnce))
  (Default|SetEnemyDiffculty _output_get self))

(event EventTick
  (params (DeltaSeconds :type Float%20%28single-precision%29))
  (Utilities|FlowControl|Sequence
    (:then_1
      (Utilities|FlowControl|Delay 1.0)
      (Class|FVBaseCharacter|Attack))))

(event EventOnDied
  (Development|PrintString "Died")
  (Actor|DestroyActor))

(fn ConstructionScript)