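; BP_SpitterEnemy is the spitter enemy in a wave-based game, handling difficulty setup, damage feedback and death.
; On BeginPlay it caches the game instance, which sets its difficulty, and it refreshes a shooting position from the ShootingLocation component every tick.
; Taking damage briefly swaps the mesh material as a hit flash.
; On death it updates the game instance's kill counters, calls its WaveManager and destroys itself.
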(event EventOnDied
  (bind _mgi (Variables|Default|GetMGI))
  (Math|Integer|IncrementInt (Variables|/Game/BP/BP_MainGameInstasnce.BP_MainGameInstasnce_C|GetEnemies%20killed _mgi)
    (:%20%20
      (Math|Integer|IncrementInt (Variables|/Game/BP/BP_MainGameInstasnce.BP_MainGameInstasnce_C|GetSpitters%20Killed _mgi)
        (:%20%20
          (Default|WaveManager _mgi)
          (Actor|DestroyActor))))))

(event EventTick
  (params (DeltaSeconds :type Float%20%28single-precision%29))
  (Variables|Default|SetShootingPosition (Transformation|GetWorldLocation (Variables|Default|GetShootingLocation))))

(event EventBeginPlay
  (bind _asbp_main_game_instasnce (Utilities|Casting|CastToBP_MainGameInstasnce (Game|GetGameInstance)))
  (bind _output_get (Variables|Default|SetMGI _asbp_main_game_instasnce))
  (Default|SetEnemyDiffculty _output_get self)
  (Variables|Default|SetShootingPosition (Transformation|GetWorldLocation (Variables|Default|GetShootingLocation))))

(event EventOnTakenDamage
  (bind _mesh (Variables|Character|GetMesh))
  (Rendering|Material|SetMaterial _mesh 0 (Variables|Default|GetDamageMaterial))
  (Utilities|FlowControl|Delay 0.2)
  (Rendering|Material|SetMaterial _mesh 0 (Variables|Default|GetNormalMaterial)))

(fn ConstructionScript)