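; BP_HunterEnemy is a hunter enemy character that reacts to being hurt, attacking the player and dying.
; Damage prints its Health and plays a hurt montage, while attacking plays a pin-down montage.
; On death it disables capsule collision, clears the anim class and ragdolls the mesh through physics simulation.
; It also calls Stun for the same seven seconds it waits before destroying itself.
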(event EventOnTakenDamage
  (Development|PrintString (Utilities|String|ToString(Float) (Variables|Default|GetHealth)))
  (Animation|PlayAnimMontage "/Game/LevelPrototyping/Characters/Enemy/walkcycle_rig_enemy-hurt_Montage.walkcycle_rig_enemy-hurt_Montage" 1.0 "None"))

(event EventOnAttackPlayer
  (Animation|PlayAnimMontage "/Game/LevelPrototyping/Characters/Enemy/walkcycle_rig_enemy-pindown_Montage.walkcycle_rig_enemy-pindown_Montage" 1.0 "None"))

(event EventOnDied
  (Collision|SetCollisionEnabled (Variables|Default|GetCapsuleComponent) "NoCollision")
  (Class|SkeletalMeshComponent|SetAnimClass (Variables|Character|GetMesh))
  (Physics|SetSimulatePhysics (Variables|Character|GetMesh) true)
  (Class|FVEnemyBase|Stun 7.0)
  (Utilities|FlowControl|Delay 7.0)
  (Actor|DestroyActor))

(fn ConstructionScript)