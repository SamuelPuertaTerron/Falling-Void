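; BP_TankEnemy is an enemy that deals contact damage to the robot and samurai players, scaled by the game instance's damage boost.
; On spawn it has the game instance set its difficulty, and on death it requests a drop chance at its location.
; A raised robot shield absorbs the hit and hurts the tank, while a samurai parry stuns it.
; Timed material swaps show stun and damage feedback.
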(event OnComponentBeginOverlap(CollisionComponent)
  (params (OverlappedComponent :type Primitive%20Component%20Object%20Reference) (OtherActor :type Actor%20Object%20Reference) (OtherComp :type Primitive%20Component%20Object%20Reference) (OtherBodyIndex :type Integer) (bFromSweep :type Boolean) (SweepResult :type Hit%20Result%20Structure%20%28by%20ref%29))
  (bind _mesh (Variables|Character|GetMesh))
  (bind _basedamage (Variables|Default|GetBaseDamage))
  (bind _mgi (Variables|Default|GetMGI))
  (bind _enemy_dmg_boost (Variables|/Game/BP/BP_MainGameInstasnce.BP_MainGameInstasnce_C|GetEnemy%20Dmg%20Boost _mgi))
  (bind _returnvalue (* _basedamage _enemy_dmg_boost))
  (bind _asbp_player_robot (Utilities|Casting|CastToBP_PlayerRobot OtherActor)
    (:then
      (if (and (== (Variables|/Game/BP/BP_PlayerRobot.BP_PlayerRobot_C|GetShield _asbp_player_robot) OtherComp) (Variables|/Script/FallingVoid.FVPlayerRobot|GetIsShielding _asbp_player_robot))
        (Default|ShieldDamage _asbp_player_robot _returnvalue)
        (Class|FVBaseCharacter|TakeDamage 1e+01)
        (else
          (Class|FVBaseCharacter|TakeDamage _asbp_player_robot _returnvalue))))
    (:CastFailed
      (bind _asbp_player_samurai (Utilities|Casting|CastToBP_PlayerSamurai OtherActor))
      (if (Variables|/Game/BP/BP_PlayerSamurai.BP_PlayerSamurai_C|GetParrying _asbp_player_samurai)
        (Class|FVEnemyBase|Stun 2.0)
        (Rendering|Material|SetMaterial _mesh 0 "/Game/Materials/M_Blue.M_Blue")
        (Utilities|FlowControl|Delay 2.0)
        (Rendering|Material|SetMaterial _mesh 0 "/Game/Materials/M_Orange.M_Orange")
        (else
          (Class|FVBaseCharacter|TakeDamage _asbp_player_samurai _returnvalue))))))

(event EventOnDied
  (Default|DropChance (Variables|Default|GetMGI) (Transformation|GetActorLocation))
  (Actor|DestroyActor))

(event EventBeginPlay
  (bind _asbp_main_game_instasnce (Utilities|Casting|CastToBP_MainGameInstasnce (Game|GetGameInstance)))
  (bind _output_get (Variables|Default|SetMGI _asbp_main_game_instasnce))
  (Utilities|FlowControl|Delay 0.2)
  (Default|SetEnemyDiffculty _output_get self))

(event EventOnTakenDamage
  (bind _mesh (Variables|Character|GetMesh))
  (Rendering|Material|SetMaterial _mesh 0 (Variables|Default|GetDamageMaterial))
  (Utilities|FlowControl|Delay 0.2)
  (Rendering|Material|SetMaterial _mesh 0 (Variables|Default|GetNormalMaterial)))

(fn ConstructionScript)