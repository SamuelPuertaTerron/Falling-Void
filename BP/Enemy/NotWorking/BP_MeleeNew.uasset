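; BP_MeleeNew is a melee enemy Blueprint, filed under a NotWorking folder, that reports into the game instance's difficulty and wave tracking.
; On BeginPlay it caches BP_MainGameInstasnce and passes itself to SetEnemyDiffculty.
; On death it increments the total and melee kill counters, calls WaveManager on the game instance, then destroys itself.
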(event EventOnDied
  (bind _mgi (Variables|Default|GetMGI))
  (Math|Integer|IncrementInt (Variables|/Game/BP/BP_MainGameInstasnce.BP_MainGameInstasnce_C|GetEnemies%20killed _mgi)
    (:%20%20
      (Math|Integer|IncrementInt (Variables|/Game/BP/BP_MainGameInstasnce.BP_MainGameInstasnce_C|GetMelees%20Killed _mgi)
        (:%20%20
          (Default|WaveManager _mgi)
          (Actor|DestroyActor))))))

(event EventBeginPlay
  (bind _asbp_main_game_instasnce (Utilities|Casting|CastToBP_MainGameInstasnce (Game|GetGameInstance)))
  (bind _output_get (Variables|Default|SetMGI _asbp_main_game_instasnce))
  (Default|SetEnemyDiffculty _output_get self))

(fn ConstructionScript)