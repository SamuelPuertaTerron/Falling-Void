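; Spitter enemy projectile that damages what it hits, usually leaves a BP_SpitterAcid behind, and then destroys itself.
; The Hit event casts the target in turn to robot, samurai and bubble.
; Robot body and samurai hits apply damage and pass the player to the spawned acid; other surfaces just get acid.
; Robot shield and bubble hits take damage without acid, and a depleted bubble is destroyed.
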(event Collision|EventHit
  (params (MyComp :type Primitive%20Component%20Object%20Reference) (Other :type Actor%20Object%20Reference) (OtherComp :type Primitive%20Component%20Object%20Reference) (bSelfMoved :type Boolean) (HitLocation :type Vector :default "0, 0, 0") (HitNormal :type Vector :default "0, 0, 0") (NormalImpulse :type Vector :default "0, 0, 0") (Hit :type Hit%20Result%20Structure%20%28by%20ref%29))
  (bind _returnvalue (Transformation|GetActorRotation))
  (bind _returnvalue_2 (Transformation|GetActorLocation))
  (bind _damage (Variables|Default|GetDamage))
  (bind _asbp_player_robot (Utilities|Casting|CastToBP_PlayerRobot Other)
    (:then
      (if (!= OtherComp (Variables|/Game/BP/BP_PlayerRobot.BP_PlayerRobot_C|GetShield _asbp_player_robot))
        (Class|FVBaseCharacter|TakeDamage _asbp_player_robot _damage)
        (bind _returnvalue_3 (Game|SpawnActorfromClass "/Game/BP/Enemy/BP_SpitterAcid.BP_SpitterAcid_C" (Math|Transform|MakeTransform _returnvalue_2 (Math|Rotator|MakeRotator 0.0 0.0 (.yaw _returnvalue)) "1.000000,1.000000,1.000000") "AdjustIfPossibleButAlwaysSpawn" "MultiplyWithRoot" 0 0))
        (Variables|/Game/BP/Enemy/BP_SpitterAcid.BP_SpitterAcid_C|SetAs%20BP%20Player%20Robot _returnvalue_3 _asbp_player_robot)
        (Actor|DestroyActor :!label _label)
        (else
          (Default|ShieldDamage _asbp_player_robot _damage)
          (Actor|DestroyActor))))
    (:CastFailed
      (bind _asbp_player_samurai (Utilities|Casting|CastToBP_PlayerSamurai Other)
        (:then
          (Class|FVBaseCharacter|TakeDamage _asbp_player_samurai _damage)
          (bind _returnvalue_4 (Game|SpawnActorfromClass "/Game/BP/Enemy/BP_SpitterAcid.BP_SpitterAcid_C" (Math|Transform|MakeTransform _returnvalue_2 (Math|Rotator|MakeRotator 0.0 0.0 (.yaw _returnvalue)) "1.000000,1.000000,1.000000") "AdjustIfPossibleButAlwaysSpawn" "MultiplyWithRoot" 0 0))
          (Variables|/Game/BP/Enemy/BP_SpitterAcid.BP_SpitterAcid_C|SetAs%20BP%20Player%20Samurai _returnvalue_4 _asbp_player_samurai)
          (goto _label))
        (:CastFailed
          (bind _asbp_bubble (Utilities|Casting|CastToBP_Bubble Other)
            (:then
              (bind _output_get (Variables|/Game/BP/BP_Bubble.BP_Bubble_C|SetHealth _asbp_bubble (- (Variables|/Game/BP/BP_Bubble.BP_Bubble_C|GetHealth _asbp_bubble) (Variables|Default|GetDamage))))
              (if (<= _output_get 0.0)
                (Actor|DestroyActor _asbp_bubble))
              (Actor|DestroyActor))
            (:CastFailed
              (Game|SpawnActorfromClass "/Game/BP/Enemy/BP_SpitterAcid.BP_SpitterAcid_C" (Math|Transform|MakeTransform _returnvalue_2 (Math|Rotator|MakeRotator 0.0 0.0 (.yaw _returnvalue)) "1.000000,1.000000,1.000000") "AdjustIfPossibleButAlwaysSpawn" "MultiplyWithRoot" 0 0)
              (goto _label))))))))

(fn ConstructionScript)