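; Melee enemy character that damages players and bubbles on collision overlap, then drops loot and despawns after death.
; On spawn it gets difficulty settings from the game instance, whose damage boost scales hits on players.
; The robot's active shield absorbs hits and hurts the enemy, while a samurai parry stuns it.
; Material swaps and montages give feedback; the old Tick line-trace lunge attack is deprecated and disconnected.
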(event OnComponentBeginOverlap(CollisionComponent)
  (params (OverlappedComponent :type Primitive%20Component%20Object%20Reference) (OtherActor :type Actor%20Object%20Reference) (OtherComp :type Primitive%20Component%20Object%20Reference) (OtherBodyIndex :type Integer) (bFromSweep :type Boolean) (SweepResult :type Hit%20Result%20Structure%20%28by%20ref%29))
  (bind _mesh (Variables|Character|GetMesh))
  (bind _basedamage (Variables|Default|GetBaseDamage))
  (bind _mgi (Variables|Default|GetMGI))
  (bind _enemy_dmg_boost (Variables|/Game/BP/BP_MainGameInstasnce.BP_MainGameInstasnce_C|GetEnemy%20Dmg%20Boost _mgi))
  (bind _returnvalue (* _basedamage _enemy_dmg_boost))
  (bind _asbp_bubble (Utilities|Casting|CastToBP_Bubble OtherActor)
    (:then
      (bind _output_get (Variables|/Game/BP/BP_Bubble.BP_Bubble_C|SetHealth _asbp_bubble (- (Variables|/Game/BP/BP_Bubble.BP_Bubble_C|GetHealth _asbp_bubble) (Variables|Default|GetBaseDamage))))
      (if (<= _output_get 0.0)
        (Actor|DestroyActor _asbp_bubble)))
    (:CastFailed
      (bind _asbp_player_robot (Utilities|Casting|CastToBP_PlayerRobot OtherActor)
        (:then
          (if (and (== (Variables|/Game/BP/BP_PlayerRobot.BP_PlayerRobot_C|GetShield _asbp_player_robot) OtherComp) (Variables|/Script/FallingVoid.FVPlayerRobot|GetIsShielding _asbp_player_robot))
            (Default|ShieldDamage _asbp_player_robot _returnvalue)
            (Class|FVBaseCharacter|TakeDamage 1e+01)
            (else
              (Class|FVBaseCharacter|TakeDamage _asbp_player_robot _returnvalue)))
          (Animation|PlayAnimMontage (.OutItem (Utilities|Array|Random (Variables|Enemy|GetAnim%20Montage))) 1.0 "None" :!label _label))
        (:CastFailed
          (bind _asbp_player_samurai (Utilities|Casting|CastToBP_PlayerSamurai OtherActor))
          (if (Variables|/Game/BP/BP_PlayerSamurai.BP_PlayerSamurai_C|GetParrying _asbp_player_samurai)
            (Class|FVEnemyBase|Stun (Variables|/Game/BP/BP_PlayerSamurai.BP_PlayerSamurai_C|GetParryStunTime _asbp_player_samurai))
            (Rendering|Material|SetMaterial _mesh 0 "/Game/Materials/M_Blue.M_Blue")
            (Utilities|FlowControl|Delay (Variables|/Game/BP/BP_PlayerSamurai.BP_PlayerSamurai_C|GetParryStunTime _asbp_player_samurai))
            (Rendering|Material|SetMaterial _mesh 0 "/Game/Materials/M_Orange.M_Orange")
            (else
              (Class|FVBaseCharacter|TakeDamage _asbp_player_samurai _returnvalue)
              (goto _label))))))))

(event EventTick
  (params (DeltaSeconds :type Float%20%28single-precision%29))
  ;[0.5 0 0] Depecated
)

(event EventOnDied
  (Default|DropChance (Variables|Default|GetMGI) (Transformation|GetActorLocation))
  (Physics|SetSimulatePhysics (Variables|Character|GetMesh) false)
  (Utilities|FlowControl|Delay 7.0)
  (Actor|DestroyActor))

(event EventBeginPlay
  (bind _asbp_main_game_instasnce (Utilities|Casting|CastToBP_MainGameInstasnce (Game|GetGameInstance)))
  (Variables|Default|SetMGI _asbp_main_game_instasnce)
  (Utilities|FlowControl|Delay 0.2)
  (Default|SetEnemyDiffculty _asbp_main_game_instasnce self))

(event EventOnTakenDamage
  (bind _mesh (Variables|Character|GetMesh))
  (Rendering|Material|SetMaterial _mesh 0 (Variables|Default|GetDamageMaterial))
  (Utilities|FlowControl|Delay 0.2)
  (Rendering|Material|SetMaterial _mesh 0 (Variables|Default|GetNormalMaterial))
  (Animation|PlayAnimMontage "/Game/LevelPrototyping/Characters/Enemy/walkcycle_rig_enemy-hurt_Montage.walkcycle_rig_enemy-hurt_Montage" 1.0 "None")
  (Development|PrintString (Utilities|String|ToString(Float) (Variables|Default|GetHealth))))

(fn ConstructionScript)