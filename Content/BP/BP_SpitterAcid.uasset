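; Acid hazard, likely from a spitter, that drops to the floor, spreads into a flat puddle and damages players standing in it.
; Repeated downward force settles the physics box for half a second, then physics stops and a timeline widens the acid cube.
; Overlaps start Delay-based damage loops tracked separately for Robot and Samurai players, ending on exit.
; The actor destroys itself five seconds after growth finishes.
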(event OnComponentBeginOverlap(Box)
  (params (OverlappedComponent :type Primitive%20Component%20Object%20Reference) (OtherActor :type Actor%20Object%20Reference) (OtherComp :type Primitive%20Component%20Object%20Reference) (OtherBodyIndex :type Integer) (bFromSweep :type Boolean) (SweepResult :type Hit%20Result%20Structure%20%28by%20ref%29))
  (bind _damage_per_tick (Variables|Default|GetDamage%20per%20tick))
  (bind _tick (Variables|Default|GetTick))
  (bind _active (Variables|Default|GetActive))
  (bind _asbp_player_robot (Utilities|Casting|CastToBP_PlayerRobot OtherActor)
    (:then
      (bind _output_get (Variables|Default|SetAs%20BP%20Player%20Robot _asbp_player_robot))
      (bind _output_get_2 (Variables|Default|SetRobot true))
      (if _active
        (Class|FVBaseCharacter|TakeDamage _output_get _damage_per_tick :!label _label)
        (Utilities|FlowControl|Delay _tick :!label _label_2)
        (if _output_get_2
          (goto _label))
        (else
          (goto _label_2))))
    (:CastFailed
      (bind _asbp_player_samurai (Utilities|Casting|CastToBP_PlayerSamurai OtherActor))
      (bind _output_get_3 (Variables|Default|SetAs%20BP%20Player%20Samurai _asbp_player_samurai))
      (bind _output_get_4 (Variables|Default|SetSamurai true))
      (if _active
        (Class|FVBaseCharacter|TakeDamage _output_get_3 _damage_per_tick :!label _label_3)
        (Utilities|FlowControl|Delay _tick :!label _label_4)
        (if _output_get_4
          (goto _label_3))
        (else
          (goto _label_4))))))

(event OnComponentEndOverlap(Box)
  (params (OverlappedComponent :type Primitive%20Component%20Object%20Reference) (OtherActor :type Actor%20Object%20Reference) (OtherComp :type Primitive%20Component%20Object%20Reference) (OtherBodyIndex :type Integer))
  (Utilities|Casting|CastToBP_PlayerRobot OtherActor
    (:then
      (Variables|Default|SetRobot false))
    (:CastFailed
      (Utilities|Casting|CastToBP_PlayerSamurai OtherActor)
      (Variables|Default|SetSamurai false))))

(event EventBeginPlay
  (Utilities|FlowControl|Sequence
    (:then_0
      (Utilities|FlowControl|Delay 0.5)
      (Variables|Default|SetActive true)
      (Physics|SetSimulatePhysics (Variables|Default|GetBox1) false)
      (Rendering|Material|SetMaterial (Variables|Default|GetCube) 0 "/Game/Materials/M_Acid.M_Acid")
      (bind _range (Timeline|Grow PlayFromStart)
        (:Update
          (Transformation|SetWorldScale3D (Variables|Default|GetCube) (Math|Vector|MakeVector _range _range 0.01)))
        (:Finished
          (Utilities|FlowControl|Delay 5.0)
          (Variables|Default|SetRobot false)
          (Variables|Default|SetSamurai false)
          (Actor|DestroyActor))))
    (:then_1
      ;[1 1 1] Tp it to the floor (And stop it bouncing)
      (if (not (Variables|Default|GetActive)) :!label _label
        (Physics|AddForce (Variables|Default|GetBox1) "0.000000,0.000000,-1000.000000" "None" false)
        (Utilities|FlowControl|Delay 0.01)
        (goto _label)))))

(fn ConstructionScript)