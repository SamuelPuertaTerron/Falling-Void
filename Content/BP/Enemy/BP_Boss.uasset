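; BP_Boss is the AI boss enemy (Egon in its sounds) that registers with the game instance, receives difficulty scaling and triggers the win after dying.
; It feeds health and waypoint location to the blackboard and tracks a state enum, switching to Retreating when damaged while health is at least half.
; Its attack overlap damages bubbles, robot and samurai players, with shield blocks hurting the boss and parries stunning it.
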(event OnComponentBeginOverlap(Attacking)
  (params (OverlappedComponent :type Primitive%20Component%20Object%20Reference) (OtherActor :type Actor%20Object%20Reference) (OtherComp :type Primitive%20Component%20Object%20Reference) (OtherBodyIndex :type Integer) (bFromSweep :type Boolean) (SweepResult :type Hit%20Result%20Structure%20%28by%20ref%29))
  (bind _basedamage (Variables|Default|GetBaseDamage))
  (bind _mgi (Variables|Default|GetMGI))
  (bind _enemy_dmg_boost (Variables|/Game/BP/BP_MainGameInstasnce.BP_MainGameInstasnce_C|GetEnemy%20Dmg%20Boost _mgi))
  (bind _returnvalue (* _basedamage _enemy_dmg_boost))
  (bind _asbp_bubble (Utilities|Casting|CastToBP_Bubble OtherActor)
    (:then
      (bind _output_get (Variables|/Game/BP/BP_Bubble.BP_Bubble_C|SetHealth _asbp_bubble (- (Variables|/Game/BP/BP_Bubble.BP_Bubble_C|GetHealth _asbp_bubble) (Variables|Default|GetBaseDamage))))
      (if (<= _output_get 0.0)
        (Actor|DestroyActor _asbp_bubble)))
    (:CastFailed
      (bind _asbp_player_robot (Utilities|Casting|CastToBP_PlayerRobot OtherActor)
        (:then
          (if (and (== (Variables|/Game/BP/BP_PlayerRobot.BP_PlayerRobot_C|GetShield _asbp_player_robot) OtherComp) (Variables|/Script/FallingVoid.FVPlayerRobot|GetIsShielding _asbp_player_robot))
            (Default|ShieldDamage _asbp_player_robot _returnvalue)
            (Class|FVBaseCharacter|TakeDamage 1e+01)
            (else
              (Class|FVBaseCharacter|TakeDamage _asbp_player_robot _returnvalue)
              (Audio|PlaySoundatLocation "/Game/Sounds/FX/Egon/Sound_EgonAttackContact.Sound_EgonAttackContact" (Transformation|GetActorLocation) "0, 0, 0" 1.0 1.0 0.0 0 0 0 0 :!label _label))))
        (:CastFailed
          (bind _asbp_player_samurai (Utilities|Casting|CastToBP_PlayerSamurai OtherActor))
          (if (Variables|/Game/BP/BP_PlayerSamurai.BP_PlayerSamurai_C|GetParrying _asbp_player_samurai)
            (Class|FVEnemyBase|Stun (Variables|/Game/BP/BP_PlayerSamurai.BP_PlayerSamurai_C|GetParryStunTime _asbp_player_samurai))
            ;[1 1 1] Doesnt work idk why
            (bind _returnvalue_2 (Niagara|SpawnSystematLocation "/Game/FX/Dylans/Stunned/DazedEnemy/Dazed.Dazed" (+ (Transformation|GetWorldLocation (Variables|Character|GetMesh)) "30.000000,0.000000,50.000000") "0, 0, 0" "1.000000,1.000000,1.000000" true true "AutoRelease"))
            (Utilities|FlowControl|Delay (Variables|/Game/BP/BP_PlayerSamurai.BP_PlayerSamurai_C|GetParryStunTime _asbp_player_samurai))
            (Components|DestroyComponent _returnvalue_2)
            (else
              (Class|FVBaseCharacter|TakeDamage _asbp_player_samurai _returnvalue)
              (goto _label))))))))

(event Custom|MoveToWaypoint
  (bind _returnvalue (Actor|GetActorOfClass "/Game/BP/Enemy/AI/BP_Waypoint.BP_Waypoint_C"))
  (AI|Components|Blackboard|SetValueasVector (AI|GetBlackboard (AI|GetAIController (Pawn|GetController))) (Variables|Default|GetKey%20Name) (Transformation|GetActorLocation _returnvalue)))

(event EventOnAttackPlayer
  (Utilities|FlowControl|Delay 2.0)
  (Class|FVBossEnemy|ResetCollision))

(event EventOnDied
  ;[1 1 1] Add Credits
  (Variables|Default|SetBossState "Dead")
  (Collision|SetCollisionEnabled (Variables|Character|GetMesh) "NoCollision")
  (Collision|SetCollisionEnabled (Variables|Default|GetCapsuleComponent) "NoCollision")
  (Audio|PlaySoundatLocation "/Game/Sounds/FX/Egon/Sound_EgonDeath.Sound_EgonDeath" (Transformation|GetActorLocation) "0, 0, 0" 1.0 1.0 0.0 0 0 0 0)
  (Utilities|FlowControl|Delay 2.5)
  (Default|Winning (Variables|Default|GetMGI)))

(event EventBeginPlay
  (bind _asbp_main_game_instasnce (Utilities|Casting|CastToBP_MainGameInstasnce (Game|GetGameInstance)))
  (bind _output_get (Variables|Default|SetMGI _asbp_main_game_instasnce))
  (Default|SetBoss _output_get self)
  (Default|OnBossSpawn (Variables|/Game/BP/BP_MainGameInstasnce.BP_MainGameInstasnce_C|GetBossSpawnManager _asbp_main_game_instasnce))
  (Utilities|FlowControl|Delay 0.2)
  (Default|SetEnemyDiffculty _asbp_main_game_instasnce self)
  (Variables|Default|SetCollisionComponent (Variables|Default|GetAttacking))
  (AI|Components|Blackboard|SetValueasFloat (AI|GetBlackboard (Pawn|GetController)) (Variables|Default|GetKey%20NameHealth) (Variables|Default|GetHealth))
  (Variables|Default|SetBossState "Moving"))

(event EventOnTakenDamage
  ;[1 1 1] Add Credits
  (Audio|PlaySoundatLocation "/Game/Sounds/FX/Egon/Sound_EgonGrunt.Sound_EgonGrunt" (Transformation|GetActorLocation) "0, 0, 0" 1.0 1.0 0.0 0 0 0 0)
  (AI|Components|Blackboard|SetValueasFloat (Variables|/Script/AIModule.AIController|GetBlackboard (AI|GetAIController self)) (Variables|Default|GetKey%20NameHealth) (Variables|Default|GetHealth))
  (if (<= (/ (Variables|Default|GetMaxHealth) 2.0) (Variables|Default|GetHealth))
    (Variables|Default|SetBossState "Retreating")))

(event EventOnAttackBegin)

(event EventTick
  (params (DeltaSeconds :type Float%20%28single-precision%29))
  (Development|PrintString (Utilities|String|EnumtoString (Variables|Default|GetBossState))))

(fn ConstructionScript)