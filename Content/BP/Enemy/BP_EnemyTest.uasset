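; Test enemy that periodically turns to face the player robot and attacks it.
; BeginPlay caches player 0's character as a BP_PlayerRobot.
; Tick runs through a one-second Delay, so roughly once a second it snaps to a look-at rotation toward that robot and calls Attack, which is not defined in this graph.
; On death it prints a debug message and destroys itself.
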(event EventBeginPlay
  (bind _asbp_player_robot (Utilities|Casting|CastToBP_PlayerRobot (Game|GetPlayerCharacter 0)))
  (Variables|Default|SetAs%20BP%20Player%20Robot _asbp_player_robot))

(event EventTick
  (params (DeltaSeconds :type Float%20%28single-precision%29))
  (Utilities|FlowControl|Delay 1.0)
  (Transformation|SetActorRotation (Math|Rotator|FindLookatRotation (Transformation|GetActorLocation) (Transformation|GetActorLocation (Variables|Default|GetAs%20BP%20Player%20Robot))))
  (Class|FVBaseCharacter|Attack))

(event EventOnDied
  (Development|PrintString "Died")
  (Actor|DestroyActor))

(fn ConstructionScript)