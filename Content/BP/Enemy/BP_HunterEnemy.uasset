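; Hunter enemy Blueprint that pins down a player and deals repeated damage while the pin holds.
; On attack it plays a pin-down montage and targets the nearer of up to two players, then Tick applies throttled damage and enables custom depth while pinned.
; Events drive hit flashes, stun FX and death with ragdoll, sound and drop chance.
; The game instance sets its difficulty shortly after spawn.
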(event EventOnTakenDamage
  (bind _mesh (Variables|Character|GetMesh))
  (Animation|PlayAnimMontage "/Game/LevelPrototyping/Characters/Enemy/walkcycle_rig_enemy-hurt_Montage.walkcycle_rig_enemy-hurt_Montage" 1.0 "None")
  (Rendering|Material|SetMaterial _mesh 0 (Variables|Default|GetDamageMaterial))
  (Utilities|FlowControl|Delay 0.2)
  (Rendering|Material|SetMaterial _mesh 0 (Variables|Default|GetNormalMaterial)))

(event EventOnAttackPlayer
  (bind _returnvalue (Transformation|GetActorLocation))
  (Animation|PlayAnimMontage "/Game/LevelPrototyping/Characters/Enemy/walkcycle_rig_enemy-pindown_Montage.walkcycle_rig_enemy-pindown_Montage" 1.0 "None")
  (bind _outactors (Actor|GetAllActorsOfClass "/Script/FallingVoid.FVPlayerBase"))
  (Utilities|IsValid (Utilities|Array|Get(acopy) _outactors 1)
    (:Is%20Valid
      (if (< (Math|Vector|Distance(Vector) (Transformation|GetActorLocation (Utilities|Array|Get(acopy) _outactors)) _returnvalue) (Math|Vector|Distance(Vector) (Transformation|GetActorLocation (Utilities|Array|Get(acopy) _outactors 1)) _returnvalue))
        (Variables|Default|SetPlayerToAttack (Utilities|Array|Get(acopy) _outactors) :!label _label)
        (else
          (Variables|Default|SetPlayerToAttack (Utilities|Array|Get(acopy) _outactors 1)))))
    (:Is%20Not%20Valid
      (goto _label))))

(event EventOnDied
  (bind _returnvalue (Transformation|GetActorLocation))
  (Game|SpawnActorfromClass "/Game/BP/Enemy/BP_Ragdoll.BP_Ragdoll_C" (Transformation|GetActorTransform) "AlwaysSpawn" "MultiplyWithRoot" 0 3 0)
  (Class|FVHunterEnemy|SetPlayerAlive)
  (Default|DropChance (Variables|Default|GetMGI) _returnvalue)
  (Audio|PlaySoundatLocation "/Game/Sounds/FX/Enemy/Sound_EnemyDeath.Sound_EnemyDeath" _returnvalue "0, 0, 0" 1.0 1.0 0.0 0 0 0 0)
  (Actor|DestroyActor))

(event EventTick
  (params (DeltaSeconds :type Float%20%28single-precision%29))
  (if (Variables|Default|GetIsPlayerPinned)
    (Utilities|FlowControl|DoOnce false :!label _label
      (:Completed
        (Class|FVBaseCharacter|TakeDamage (Variables|Default|GetPlayerToAttack) 1e+01)
        (Rendering|SetRenderCustomDepth (Variables|Character|GetMesh) true)
        (Utilities|FlowControl|Delay 0.5)
        (goto _label Reset)))
    (else
      (Rendering|SetRenderCustomDepth (Variables|Character|GetMesh) false))))

(event EventBeginPlay
  (bind _asbp_main_game_instasnce (Utilities|Casting|CastToBP_MainGameInstasnce (Game|GetGameInstance)))
  (Variables|Default|SetMGI _asbp_main_game_instasnce)
  (Utilities|FlowControl|Delay 0.2)
  (Default|SetEnemyDiffculty _asbp_main_game_instasnce self))

(event EventOnStunStart
  (Rendering|SetVisibility (Variables|Default|GetStunFX) true false))

(event EventOnStunEnd
  (Rendering|SetVisibility (Variables|Default|GetStunFX) false false))

(fn ConstructionScript)