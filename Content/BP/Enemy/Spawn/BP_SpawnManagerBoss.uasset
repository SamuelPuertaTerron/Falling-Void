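; Boss-fight spawn manager that alternates the boss between the arena and waves of enemies.
; It registers with the game instance, then on boss spawn caches the boss, spawn points and hiding spot.
; BossClear moves the boss to the hiding spot and spawns random enemy classes at random points.
; Destroy events count enemies down, returning the boss to the world origin in Moving state when none remain.
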(event Custom|Boss%20Clear
  (bind _boss (Variables|Default|GetBoss))
  (Utilities|Casting|CastToBP__EnemyAI (AI|GetAIController _boss))
  (Transformation|SetActorLocation _boss (Variables|Default|GetBossHidingStop) false false)
  (CallFunction|SpawnWave 1)
  (Variables|/Script/FallingVoid.FVBossEnemy|SetBossState _boss "Jumping"))

(event Custom|Boss%20Returns
  (bind _boss (Variables|Default|GetBoss))
  (Transformation|SetActorLocation _boss "0, 0, 0" false false)
  (Variables|/Script/FallingVoid.FVBossEnemy|SetBossState _boss "Moving"))

(event Custom|SpawnWave
  (params (MaxEnemies :type Integer))
  (for _index (range 0 MaxEnemies)
    (bind _returnvalue (Game|SpawnActorfromClass (.OutItem (Utilities|Array|Random (Variables|Default|GetEnemyClass))) (Math|Transform|MakeTransform (Transformation|GetActorLocation (.OutItem (Utilities|Array|Random (Variables|Default|GetSpawnPoints)))) "0, 0, 0" "1.000000,1.000000,1.000000") "Undefined" "MultiplyWithRoot" 0 0))
    (Math|Integer|IncrementInt (Variables|Default|GetCurrentEnemyCount)
      (:%20%20
        (Utilities|IsValid _returnvalue
          (:Is%20Valid
            (Game|BindEventtoOnDestroyed _returnvalue (delegate Custom|EnemyOnDeath))))))))

(event Custom|EnemyOnDeath
  (params (DestroyedActor :type Actor%20Object%20Reference))
  (bind _currentenemycount (Variables|Default|GetCurrentEnemyCount))
  (Math|Integer|DecrementInt _currentenemycount
    (:%20%20
      (if (<= _currentenemycount 0)
        (CallFunction|BossReturns)))))

(event Custom|OnBossSpawn
  (bind _asbp_main_game_instasnce (Utilities|Casting|CastToBP_MainGameInstasnce (Game|GetGameInstance)))
  (Variables|Default|SetBoss (Variables|/Game/BP/BP_MainGameInstasnce.BP_MainGameInstasnce_C|GetBoss _asbp_main_game_instasnce))
  (bind _outactors (Actor|GetAllActorsOfClass "/Game/BP/Enemy/Spawn/BP_SpawnPointBoss.BP_SpawnPointBoss_C"))
  (Variables|Default|SetSpawnPoints _outactors)
  (bind _returnvalue (Actor|GetActorOfClass "/Game/BP/Enemy/Spawn/BP_BossHidingSpot.BP_BossHidingSpot_C"))
  (Variables|Default|SetBossHidingStop (Transformation|GetActorLocation _returnvalue))
  (CallFunction|BossReturns))

(event EventBeginPlay
  (bind _asbp_main_game_instasnce (Utilities|Casting|CastToBP_MainGameInstasnce (Game|GetGameInstance)))
  (Variables|/Game/BP/BP_MainGameInstasnce.BP_MainGameInstasnce_C|SetBossSpawnManager _asbp_main_game_instasnce self))

(fn ConstructionScript)