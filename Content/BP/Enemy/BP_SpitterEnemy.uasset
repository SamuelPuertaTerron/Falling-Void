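; BP_SpitterEnemy is a spitter enemy that reacts to attack, damage and death events.
; On BeginPlay it caches the game instance and, after a short delay, passes itself to it for difficulty setup.
; Tick keeps ShootingPosition synced to the ShootingLocation component, while attacks only play the spit montage here.
; Damage briefly swaps the mesh material as a hit flash, and death asks the game instance for a drop chance before destroying the actor.
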(event EventOnDied
  (Default|DropChance (Variables|Default|GetMGI) (Transformation|GetActorLocation))
  (Actor|DestroyActor))

(event EventTick
  (params (DeltaSeconds :type Float%20%28single-precision%29))
  (Variables|Default|SetShootingPosition (Transformation|GetWorldLocation (Variables|Default|GetShootingLocation))))

(event EventBeginPlay
  (bind _asbp_main_game_instasnce (Utilities|Casting|CastToBP_MainGameInstasnce (Game|GetGameInstance)))
  (bind _output_get (Variables|Default|SetMGI _asbp_main_game_instasnce))
  (Utilities|FlowControl|Delay 0.2)
  (Default|SetEnemyDiffculty _output_get self)
  (Variables|Default|SetShootingPosition (Transformation|GetWorldLocation (Variables|Default|GetShootingLocation))))

(event EventOnAttackPlayer
  (Animation|PlayAnimMontage "/Game/LevelPrototyping/Characters/Enemy/walkcycle_rig_enemy-spit_Montage.walkcycle_rig_enemy-spit_Montage" 1.0 "None"))

(event EventOnTakenDamage
  (bind _mesh (Variables|Character|GetMesh))
  (Rendering|Material|SetMaterial _mesh 0 (Variables|Default|GetDamageMaterial))
  (Utilities|FlowControl|Delay 0.2)
  (Rendering|Material|SetMaterial _mesh 0 (Variables|Default|GetNormalMaterial)))

(fn ConstructionScript)