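; BP_Ragdoll is a short-lived physics corpse for a dead enemy, covering Runt, Brute, Spitter and Prowler variants.
; On BeginPlay it switches on DeadEnemy to apply the matching material to its skeletal mesh, also scaling the mesh up for the Brute.
; It then enables physics simulation on the mesh and destroys itself after a fixed delay.
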(event EventBeginPlay
  (bind _skeletalmesh (Variables|Default|GetSkeletalMesh))
  (switch int (Variables|Default|GetDead%20Enemy)
    (:0
      (Rendering|Material|SetMaterial _skeletalmesh 0 "/Game/LevelPrototyping/Materials/M_Runt.M_Runt"))
    (:1
      (Rendering|Material|SetMaterial _skeletalmesh 0 "/Game/LevelPrototyping/Materials/M_Brute.M_Brute")
      (Transformation|SetRelativeScale3D (Variables|Default|GetSkeletalMesh) "1.500000,1.500000,1.500000"))
    (:2
      (Rendering|Material|SetMaterial _skeletalmesh 0 "/Game/LevelPrototyping/Materials/M_Spitter.M_Spitter"))
    (:3
      (Rendering|Material|SetMaterial _skeletalmesh 0 "/Game/LevelPrototyping/Materials/M_Prowler.M_Prowler")))
  (Physics|SetSimulatePhysics (Variables|Default|GetSkeletalMesh) true)
  (Utilities|FlowControl|Delay 5.0)
  (Actor|DestroyActor))

(fn ConstructionScript)