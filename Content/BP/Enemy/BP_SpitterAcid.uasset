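; Spitter enemy acid puddle that damages the Robot and Samurai players and BP_Bubble actors.
; On BeginPlay it is pushed down, then after half a second freezes physics, activates, shows acid material and bubbles, widens via the Grow timeline, and later self-destructs.
; Overlaps run Delay-based damage loops, which end-overlap flags stop for players.
; Bubbles have no exit check, losing Health until it drops below zero and they are destroyed.
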(event OnComponentBeginOverlap(Acid)
  (params (OverlappedComponent :type Primitive%20Component%20Object%20Reference) (OtherActor :type Actor%20Object%20Reference) (OtherComp :type Primitive%20Component%20Object%20Reference) (OtherBodyIndex :type Integer) (bFromSweep :type Boolean) (SweepResult :type Hit%20Result%20Structure%20%28by%20ref%29))
  (bind _active (Variables|Default|GetActive))
  (bind _damage_per_tick (Variables|Default|GetDamage%20per%20tick))
  (bind _tick (Variables|Default|GetTick))
  (bind _asbp_player_robot (Utilities|Casting|CastToBP_PlayerRobot OtherActor)
    (:then
      (bind _output_get (Variables|Default|SetAs%20BP%20Player%20Robot _asbp_player_robot))
      (bind _output_get_2 (Variables|Default|SetRobot true))
      (if _active
        (Class|FVBaseCharacter|TakeDamage _output_get _damage_per_tick :!label _label)
        (Utilities|FlowControl|Delay _tick :!label _label_2)
        (if _output_get_2
          (goto _label))
        (else
          (goto _label_2))))
    (:CastFailed
      (bind _asbp_player_samurai (Utilities|Casting|CastToBP_PlayerSamurai OtherActor)
        (:then
          (bind _output_get_3 (Variables|Default|SetAs%20BP%20Player%20Samurai _asbp_player_samurai))
          (bind _output_get_4 (Variables|Default|SetSamurai true))
          (if _active
            (Class|FVBaseCharacter|TakeDamage _output_get_3 _damage_per_tick :!label _label_3)
            (Utilities|FlowControl|Delay _tick :!label _label_4)
            (if _output_get_4
              (goto _label_3))
            (else
              (goto _label_4))))
        (:CastFailed
          (bind _asbp_bubble (Utilities|Casting|CastToBP_Bubble OtherActor))
          (if (Variables|Default|GetActive)
            (Utilities|IsValid _asbp_bubble :!label _label_5
              (:Is%20Valid
                (bind _output_get_5 (Variables|/Game/BP/BP_Bubble.BP_Bubble_C|SetHealth _asbp_bubble (- (Variables|/Game/BP/BP_Bubble.BP_Bubble_C|GetHealth _asbp_bubble) (Variables|Default|GetDamage%20per%20tick))))
                (if (>= _output_get_5 0.0)
                  (Utilities|FlowControl|Delay (Variables|Default|GetTick))
                  (if true
                    (goto _label_5))
                  (else
                    (Actor|DestroyActor _asbp_bubble)))))))))))

(event OnComponentEndOverlap(Acid)
  (params (OverlappedComponent :type Primitive%20Component%20Object%20Reference) (OtherActor :type Actor%20Object%20Reference) (OtherComp :type Primitive%20Component%20Object%20Reference) (OtherBodyIndex :type Integer))
  (Utilities|Casting|CastToBP_PlayerRobot OtherActor
    (:then
      (Variables|Default|SetRobot false))
    (:CastFailed
      (Utilities|Casting|CastToBP_PlayerSamurai OtherActor)
      (Variables|Default|SetSamurai false))))

(event EventBeginPlay
  (Physics|AddForce (Variables|Default|GetBox1) "0.000000,0.000000,-50.000000" "None" false)
  (Utilities|FlowControl|Delay 0.5)
  (Variables|Default|SetActive true)
  (Physics|SetSimulatePhysics (Variables|Default|GetBox1) false)
  (Rendering|Material|SetMaterial (Variables|Default|GetAcid) 0 "/Game/LevelPrototyping/Materials/M_Acid.M_Acid")
  (Niagara|SpawnSystematLocation "/Game/FX/Jolie/NS_AcidBubbles.NS_AcidBubbles" (- (Transformation|GetActorLocation) "0.000000,0.000000,75.000000") "0, 0, 0" "1.000000,1.000000,1.000000" true true "AutoRelease")
  (bind _range (Timeline|Grow PlayFromStart)
    (:Update
      (Transformation|SetWorldScale3D (Variables|Default|GetAcid) (Math|Vector|MakeVector _range _range 1.0)))
    (:Finished
      (Utilities|FlowControl|Delay 5.0)
      (Variables|Default|SetRobot false)
      (Variables|Default|SetSamurai false)
      (Actor|DestroyActor))))

(fn ConstructionScript)