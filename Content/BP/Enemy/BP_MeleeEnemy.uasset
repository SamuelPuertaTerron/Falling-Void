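; Melee enemy character that damages the player robot or samurai at close range and takes part in the wave system.
; Each Tick off cooldown, it line traces forward, ignoring other melee enemies, and deals difficulty-scaled damage, routing hits on the robot's shield to shield damage.
; A hit triggers a launch-based lunge, then holds the enemy still until cooldown ends.
; On death it updates the game instance's kill count, calls StartNextWave and destroys itself.
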(event EventTick
  (params (DeltaSeconds :type Float%20%28single-precision%29))
  (bind _returnvalue (Transformation|GetActorLocation))
  (bind _returnvalue_2 (Pawn|GetControlRotation :!class /Script/Engine.Pawn))
  (bind _basedamage (Variables|Default|GetBaseDamage))
  (bind _mgi (Variables|Default|GetMGI))
  (bind _returnvalue_3 (Math|Vector|GetForwardVector _returnvalue_2))
  (bind _enemy_dmg_boost (Variables|/Game/BP/BP_MainGameInstasnce.BP_MainGameInstasnce_C|GetEnemy%20Dmg%20Boost _mgi))
  (bind _returnvalue_4 (* _basedamage _enemy_dmg_boost))
  (if (not (Variables|Default|GetAttack%20CD))
    (bind _outactors (Actor|GetAllActorsOfClass "BP_MeleeEnemy_C"))
    (bind _outhit (Collision|LineTraceByChannel _returnvalue (+ _returnvalue (* (Math|Vector|GetForwardVector (Transformation|GetWorldRotation (Variables|Default|GetCapsuleComponent))) 1.5e+02)) "TraceTypeQuery1" false _outactors "ForOneFrame"))
    (bind _asbp_player_robot (Utilities|Casting|CastToBP_PlayerRobot (.hitactor _outhit))
      (:then
        (if (!= (Variables|/Game/BP/BP_PlayerRobot.BP_PlayerRobot_C|GetShield _asbp_player_robot) (.hitcomponent _outhit))
          (Class|FVBaseCharacter|TakeDamage _asbp_player_robot _returnvalue_4)
          (else
            (Default|ShieldDamage _asbp_player_robot _returnvalue_4))))
      (:CastFailed
        (bind _asbp_player_samurai (Utilities|Casting|CastToBP_PlayerSamurai (.hitactor _outhit)))
        (Class|FVBaseCharacter|TakeDamage _asbp_player_samurai _returnvalue_4)))
    ;[1 1 1] A lunge to the player
    (Character|LaunchCharacter (Math|Vector|MakeVector (* (.x _returnvalue_3) 2e+04) (* (.y _returnvalue_3) 2e+04) 1e+02) true true)
    (Variables|/Script/Engine.CharacterMovementComponent|SetMaxWalkSpeed (Variables|Character|GetCharacterMovement) 0.0)
    (Variables|Default|SetAttack%20CD true)
    (Utilities|FlowControl|Delay 0.1)
    (Character|LaunchCharacter (Math|Vector|MakeVector 0.0 0.0 -1e+02) true true)
    (Utilities|FlowControl|Delay 1.9)
    (Variables|Default|SetAttack%20CD false)
    (Variables|/Script/Engine.CharacterMovementComponent|SetMaxWalkSpeed (Variables|Character|GetCharacterMovement) 6e+02)))

(event EventOnDied
  (bind _mgi (Variables|Default|GetMGI))
  (Math|Integer|IncrementInt (Variables|/Game/BP/BP_MainGameInstasnce.BP_MainGameInstasnce_C|GetEnemies%20killed _mgi)
    (:%20%20
      (Default|StartNextWave? _mgi)
      (Actor|DestroyActor))))

(event EventBeginPlay
  (bind _asbp_main_game_instasnce (Utilities|Casting|CastToBP_MainGameInstasnce (Game|GetGameInstance)))
  (bind _output_get (Variables|Default|SetMGI _asbp_main_game_instasnce))
  (Default|SetEnemyDiffculty _output_get self))

(fn ConstructionScript)