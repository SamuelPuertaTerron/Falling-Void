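; Melee enemy Blueprint that registers with the game instance for difficulty scaling and, on death, updates kill counts and calls the wave manager.
; While off cooldown, Tick traces a short line forward, ignoring other melee enemies, but the result is unconnected.
; The unreached attack logic damages the robot player, its shield or the samurai, scaled by enemy damage boost, then lunges via LaunchCharacter and pauses movement during a delayed cooldown.
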(event EventTick
  (params (DeltaSeconds :type Float%20%28single-precision%29))
  (bind _returnvalue (Transformation|GetActorLocation))
  (if (not (Variables|Default|GetAttack%20CD))
    (bind _outactors (Actor|GetAllActorsOfClass "BP_MeleeEnemy_C"))
    (bind _outhit (Collision|LineTraceByChannel _returnvalue (+ _returnvalue (* (Math|Vector|GetForwardVector (Transformation|GetWorldRotation (Variables|Default|GetCapsuleComponent))) 1.5e+02)) "TraceTypeQuery1" false _outactors "None"))))

(event EventOnDied
  (bind _mgi (Variables|Default|GetMGI))
  (Math|Integer|IncrementInt (Variables|/Game/BP/BP_MainGameInstasnce.BP_MainGameInstasnce_C|GetEnemies%20killed _mgi)
    (:%20%20
      (Math|Integer|IncrementInt (Variables|/Game/BP/BP_MainGameInstasnce.BP_MainGameInstasnce_C|GetMelees%20Killed _mgi)
        (:%20%20
          (Default|WaveManager _mgi)
          (Actor|DestroyActor))))))

(event EventBeginPlay
  (bind _asbp_main_game_instasnce (Utilities|Casting|CastToBP_MainGameInstasnce (Game|GetGameInstance)))
  (bind _output_get (Variables|Default|SetMGI _asbp_main_game_instasnce))
  (Default|SetEnemyDiffculty _output_get self))

(fn ConstructionScript)