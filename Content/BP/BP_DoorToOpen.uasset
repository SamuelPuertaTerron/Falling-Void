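; Double door actor that registers itself with the main game instance on BeginPlay so other Blueprints can open it.
; The OpenDoors event sets an Open flag, then starts moving the Left and Right components.
; MoveComponentTo slides the two leaves apart and swings them in opposite directions to their open pose.
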(event Custom|OpenDoors
  (Variables|Default|SetOpen true)
  (Utilities|FlowControl|Sequence
    (:then_0
      (Components|MoveComponentTo (Variables|Default|GetLeft) "70.000000,0.000000,0.000000" "0.000000,-90.000000,0.000000" false false 0.2 false))
    (:then_1
      (Components|MoveComponentTo (Variables|Default|GetRight) "-70.000000,0.000000,0.000000" "0.000000,90.000000,0.000000" false false 0.2 false))))

(event EventBeginPlay
  (bind _asbp_main_game_instasnce (Utilities|Casting|CastToBP_MainGameInstasnce (Game|GetGameInstance)))
  (Variables|/Game/BP/BP_MainGameInstasnce.BP_MainGameInstasnce_C|SetDoorToOpen _asbp_main_game_instasnce self))

(fn ConstructionScript)