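; BP_WinningTrigger is a box trigger that ends the level in a win once both player characters, the Robot and the Samurai, stand inside it.
; On BeginPlay it registers itself with BP_MainGameInstasnce.
; Overlap begin and end events track each character's presence, and when both are inside and the game instance's DoorToOpen is open, it calls Winning on the game instance.
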(event OnComponentBeginOverlap(Box)
  (params (OverlappedComponent :type Primitive%20Component%20Object%20Reference) (OtherActor :type Actor%20Object%20Reference) (OtherComp :type Primitive%20Component%20Object%20Reference) (OtherBodyIndex :type Integer) (bFromSweep :type Boolean) (SweepResult :type Hit%20Result%20Structure%20%28by%20ref%29))
  (Utilities|Casting|CastToBP_PlayerRobot OtherActor
    (:then
      (bind _output_get (Variables|Default|SetRobot true)))
    (:CastFailed
      (Utilities|Casting|CastToBP_PlayerSamurai OtherActor)
      (bind _output_get_2 (Variables|Default|SetSamurai true))))
  (if (Math|Boolean|ANDBoolean _output_get _output_get_2 (Variables|/Game/BP/BP_DoorToOpen.BP_DoorToOpen_C|GetOpen (Variables|/Game/BP/BP_MainGameInstasnce.BP_MainGameInstasnce_C|GetDoorToOpen (Variables|Default|GetMGI))))
    (Default|Winning (Variables|Default|GetMGI))))

(event OnComponentEndOverlap(Box)
  (params (OverlappedComponent :type Primitive%20Component%20Object%20Reference) (OtherActor :type Actor%20Object%20Reference) (OtherComp :type Primitive%20Component%20Object%20Reference) (OtherBodyIndex :type Integer))
  (Utilities|Casting|CastToBP_PlayerRobot OtherActor
    (:then
      (Variables|Default|SetRobot false))
    (:CastFailed
      (Utilities|Casting|CastToBP_PlayerSamurai OtherActor)
      (Variables|Default|SetSamurai false))))

(event EventBeginPlay
  (bind _asbp_main_game_instasnce (Utilities|Casting|CastToBP_MainGameInstasnce (Game|GetGameInstance)))
  (bind _output_get (Variables|Default|SetMGI _asbp_main_game_instasnce))
  (Variables|/Game/BP/BP_MainGameInstasnce.BP_MainGameInstasnce_C|SetWinning%20Trigger _output_get self))

(fn ConstructionScript)