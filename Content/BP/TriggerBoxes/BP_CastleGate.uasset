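; BP_CastleGate is a two-leaf castle gate that can be swung open or shut.
; On BeginPlay it registers itself with the game instance and closes immediately if the current level is 3.
; GateOpen and CloseGate each set the Open flag and animate the Left and Right components with MoveComponentTo, opening more slowly than closing.
; Each event is guarded by its own DoOnce with no reset, so each runs only once.
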(event Custom|Gate%20Open
  (Utilities|FlowControl|DoOnce false
    (:Completed
      (Variables|Default|SetOpen true)
      (Utilities|FlowControl|Sequence
        (:then_0
          (Components|MoveComponentTo (Variables|Default|GetLeft) "-315.000000,0.000000,0.000000" "0.000000,-90.000000,0.000000" false false 3.0 false))
        (:then_1
          (Components|MoveComponentTo (Variables|Default|GetRight) "315.000000,0.000000,0.000000" "0.000000,90.000000,0.000000" false false 3.0 false))))))

(event Custom|CloseGate
  (Utilities|FlowControl|DoOnce false
    (:Completed
      (Variables|Default|SetOpen false)
      (Utilities|FlowControl|Sequence
        (:then_0
          (Components|MoveComponentTo (Variables|Default|GetLeft) "-315.000000,0.000000,0.000000" "0, 0, 0" false false 1.5 false))
        (:then_1
          (Components|MoveComponentTo (Variables|Default|GetRight) "315.000000,0.000000,0.000000" "0, 0, 0" false false 1.5 false))))))

(event EventBeginPlay
  (bind _asbp_main_game_instasnce (Utilities|Casting|CastToBP_MainGameInstasnce (Game|GetGameInstance)))
  (Variables|/Game/BP/BP_MainGameInstasnce.BP_MainGameInstasnce_C|SetCastleGate _asbp_main_game_instasnce self)
  (if (== (Variables|/Game/BP/BP_MainGameInstasnce.BP_MainGameInstasnce_C|GetLevel _asbp_main_game_instasnce) 3)
    (CallFunction|CloseGate)))

(fn ConstructionScript)