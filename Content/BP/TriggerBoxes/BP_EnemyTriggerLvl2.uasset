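; BP_EnemyTriggerLvl2 is a trigger volume that starts an enemy wave through the game instance's SpawnManager.
; The first overlap by either the robot or samurai player fires it once.
; The 1st flag selects wave 0, or wave 1 along with setting the manager's OpenGate flag.
; On BeginPlay it caches the game instance and destroys itself if the current Level is 3.
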(event OnComponentBeginOverlap(Box)
  (params (OverlappedComponent :type Primitive%20Component%20Object%20Reference) (OtherActor :type Actor%20Object%20Reference) (OtherComp :type Primitive%20Component%20Object%20Reference) (OtherBodyIndex :type Integer) (bFromSweep :type Boolean) (SweepResult :type Hit%20Result%20Structure%20%28by%20ref%29))
  (bind _mgi (Variables|Default|GetMGI))
  (bind _spawnmanager (Variables|/Game/BP/BP_MainGameInstasnce.BP_MainGameInstasnce_C|GetSpawnManager _mgi))
  (Utilities|Casting|CastToBP_PlayerRobot OtherActor
    (:then
      _)
    (:CastFailed
      (Utilities|Casting|CastToBP_PlayerSamurai OtherActor)))
  (Utilities|FlowControl|DoOnce false
    (:Completed
      (if (Variables|Default|Get1st?)
        (Default|SpawnWave _spawnmanager)
        (else
          (Default|SpawnWave _spawnmanager 1)
          (Variables|/Game/BP/Enemy/Spawn/BP_SpawnManager.BP_SpawnManager_C|SetOpen%20Gate? _spawnmanager true))))))

(event EventBeginPlay
  (bind _asbp_main_game_instasnce (Utilities|Casting|CastToBP_MainGameInstasnce (Game|GetGameInstance)))
  (bind _output_get (Variables|Default|SetMGI _asbp_main_game_instasnce))
  (if (== (Variables|/Game/BP/BP_MainGameInstasnce.BP_MainGameInstasnce_C|GetLevel _output_get) 3)
    (Actor|DestroyActor)))

(fn ConstructionScript)