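; BP_Level3 is a trigger box that advances the game to level 3 once both the robot and samurai players stand inside it.
; Overlap begin and end events track each character's presence with two flags.
; When both are present, it sets the GameInstance level, saves level data, opens the castle door and closes the castle gate.
; On BeginPlay it destroys itself if the saved level is already 3.
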(event OnComponentBeginOverlap(Box)
  (params (OverlappedComponent :type Primitive%20Component%20Object%20Reference) (OtherActor :type Actor%20Object%20Reference) (OtherComp :type Primitive%20Component%20Object%20Reference) (OtherBodyIndex :type Integer) (bFromSweep :type Boolean) (SweepResult :type Hit%20Result%20Structure%20%28by%20ref%29))
  (bind _mgi (Variables|Default|GetMGI))
  (Utilities|Casting|CastToBP_PlayerRobot OtherActor
    (:then
      (bind _output_get (Variables|Default|SetRobot true)))
    (:CastFailed
      (Utilities|Casting|CastToBP_PlayerSamurai OtherActor)
      (bind _output_get_2 (Variables|Default|SetSamurai true))))
  (if (and _output_get _output_get_2)
    (Variables|/Game/BP/BP_MainGameInstasnce.BP_MainGameInstasnce_C|SetLevel _mgi 3)
    (Default|LevelDataSave _mgi)
    (Default|OpenDoors (Variables|/Game/BP/BP_MainGameInstasnce.BP_MainGameInstasnce_C|GetCastleDoor _mgi))
    (Default|CloseGate (Variables|/Game/BP/BP_MainGameInstasnce.BP_MainGameInstasnce_C|GetCastleGate _mgi))))

(event OnComponentEndOverlap(Box)
  (params (OverlappedComponent :type Primitive%20Component%20Object%20Reference) (OtherActor :type Actor%20Object%20Reference) (OtherComp :type Primitive%20Component%20Object%20Reference) (OtherBodyIndex :type Integer))
  (Utilities|Casting|CastToBP_PlayerRobot OtherActor
    (:then
      (Variables|Default|SetRobot false))
    (:CastFailed
      (Utilities|Casting|CastToBP_PlayerSamurai OtherActor)
      (Variables|Default|SetSamurai false))))

(event EventBeginPlay
  (bind _asbp_main_game_instasnce (Utilities|Casting|CastToBP_MainGameInstasnce (Game|GetGameInstance)))
  (bind _output_get (Variables|Default|SetMGI _asbp_main_game_instasnce))
  (if (== (Variables|/Game/BP/BP_MainGameInstasnce.BP_MainGameInstasnce_C|GetLevel _output_get) 3)
    (Actor|DestroyActor)))

(fn ConstructionScript)