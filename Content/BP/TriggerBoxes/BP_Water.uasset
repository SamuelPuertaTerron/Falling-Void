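; BP_Water is a water trigger volume that slows the robot and samurai player characters while they overlap its Box.
; On begin overlap it casts to each player class, sets Slowed, and lowers max walk speed if the player is alive with zero InteractTime.
; On end overlap it clears Slowed and calls the player's MoveAgain, with the same logic duplicated per class.
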(event OnComponentBeginOverlap(Box)
  (params (OverlappedComponent :type Primitive%20Component%20Object%20Reference) (OtherActor :type Actor%20Object%20Reference) (OtherComp :type Primitive%20Component%20Object%20Reference) (OtherBodyIndex :type Integer) (bFromSweep :type Boolean) (SweepResult :type Hit%20Result%20Structure%20%28by%20ref%29))
  (bind _asbp_player_robot (Utilities|Casting|CastToBP_PlayerRobot OtherActor)
    (:then
      (Variables|/Game/BP/BP_PlayerRobot.BP_PlayerRobot_C|SetSlowed _asbp_player_robot true)
      (if (and (Class|FVPlayerBase|NodeGetIsAlive _asbp_player_robot) (== (Variables|/Game/BP/BP_PlayerRobot.BP_PlayerRobot_C|GetInteract%20Time _asbp_player_robot) 0.0))
        (Variables|/Script/Engine.CharacterMovementComponent|SetMaxWalkSpeed (Variables|/Script/Engine.Character|GetCharacterMovement _asbp_player_robot) 3.5e+02)))
    (:CastFailed
      (bind _asbp_player_samurai (Utilities|Casting|CastToBP_PlayerSamurai OtherActor))
      (Variables|/Game/BP/BP_PlayerSamurai.BP_PlayerSamurai_C|SetSlowed _asbp_player_samurai true)
      (if (and (Class|FVPlayerBase|NodeGetIsAlive _asbp_player_samurai) (== (Variables|/Game/BP/BP_PlayerSamurai.BP_PlayerSamurai_C|GetInteract%20Time _asbp_player_samurai) 0.0))
        (Variables|/Script/Engine.CharacterMovementComponent|SetMaxWalkSpeed (Variables|/Script/Engine.Character|GetCharacterMovement _asbp_player_samurai) 3.5e+02)))))

(event OnComponentEndOverlap(Box)
  (params (OverlappedComponent :type Primitive%20Component%20Object%20Reference) (OtherActor :type Actor%20Object%20Reference) (OtherComp :type Primitive%20Component%20Object%20Reference) (OtherBodyIndex :type Integer))
  (bind _asbp_player_robot (Utilities|Casting|CastToBP_PlayerRobot OtherActor)
    (:then
      (Variables|/Game/BP/BP_PlayerRobot.BP_PlayerRobot_C|SetSlowed _asbp_player_robot false)
      (Default|MoveAgain _asbp_player_robot))
    (:CastFailed
      (bind _asbp_player_samurai (Utilities|Casting|CastToBP_PlayerSamurai OtherActor))
      (Variables|/Game/BP/BP_PlayerSamurai.BP_PlayerSamurai_C|SetSlowed _asbp_player_samurai false)
      (Default|MoveAgain _asbp_player_samurai))))

(event EventBeginPlay)

(event Collision|EventActorBeginOverlap
  (params (OtherActor :type Actor%20Object%20Reference)))

(event EventTick
  (params (DeltaSeconds :type Float%20%28single-precision%29)))

(fn ConstructionScript)