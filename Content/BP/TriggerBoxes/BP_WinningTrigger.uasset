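; BP_WinningTrigger is the co-op level exit trigger that calls Winning on the game instance when both Robot and Samurai are inside and DoorToOpen is open.
; Box overlaps track each character and set its InObjective flag, with the win condition checked only on overlap begin.
; It registers itself with the game instance on BeginPlay.
; SetUp2ndPlayerUI assigns the PortalIcon1 widget to player two, whichever character that is.
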(event OnComponentBeginOverlap(Box)
  (params (OverlappedComponent :type Primitive%20Component%20Object%20Reference) (OtherActor :type Actor%20Object%20Reference) (OtherComp :type Primitive%20Component%20Object%20Reference) (OtherBodyIndex :type Integer) (bFromSweep :type Boolean) (SweepResult :type Hit%20Result%20Structure%20%28by%20ref%29))
  (bind _asbp_player_robot (Utilities|Casting|CastToBP_PlayerRobot OtherActor)
    (:then
      (Variables|/Game/BP/BP_PlayerRobot.BP_PlayerRobot_C|SetInObjective _asbp_player_robot true)
      (bind _output_get (Variables|Default|SetRobot true)))
    (:CastFailed
      (bind _asbp_player_samurai (Utilities|Casting|CastToBP_PlayerSamurai OtherActor))
      (Variables|/Game/BP/BP_PlayerSamurai.BP_PlayerSamurai_C|SetInObjective _asbp_player_samurai true)
      (bind _output_get_2 (Variables|Default|SetSamurai true))))
  (if (Math|Boolean|ANDBoolean _output_get _output_get_2 (Variables|/Game/BP/TriggerBoxes/BP_DoorToOpen.BP_DoorToOpen_C|GetOpen (Variables|/Game/BP/BP_MainGameInstasnce.BP_MainGameInstasnce_C|GetDoorToOpen (Variables|Default|GetMGI))))
    (Default|Winning (Variables|Default|GetMGI))))

(event OnComponentEndOverlap(Box)
  (params (OverlappedComponent :type Primitive%20Component%20Object%20Reference) (OtherActor :type Actor%20Object%20Reference) (OtherComp :type Primitive%20Component%20Object%20Reference) (OtherBodyIndex :type Integer))
  (bind _asbp_player_robot (Utilities|Casting|CastToBP_PlayerRobot OtherActor)
    (:then
      (Variables|/Game/BP/BP_PlayerRobot.BP_PlayerRobot_C|SetInObjective _asbp_player_robot false)
      (Variables|Default|SetRobot false))
    (:CastFailed
      (bind _asbp_player_samurai (Utilities|Casting|CastToBP_PlayerSamurai OtherActor))
      (Variables|/Game/BP/BP_PlayerSamurai.BP_PlayerSamurai_C|SetInObjective _asbp_player_samurai false)
      (Variables|Default|SetSamurai false))))

(event Custom|SetUp2ndPlayerUI
  (bind _returnvalue (Game|GetPlayerCharacter 1))
  (bind _portal_icon1 (Variables|Default|GetPortal%20Icon1))
  (bind _portal_icon1_2 (Variables|Default|GetPortal%20Icon1))
  (bind _asbp_player_robot (Utilities|Casting|CastToBP_PlayerRobot _returnvalue)
    (:then
      (Class|WidgetComponent|SetOwnerPlayer _portal_icon1 (Class|Widget|GetOwningLocalPlayer (Variables|/Game/BP/BP_MainGameInstasnce.BP_MainGameInstasnce_C|GetP2%20UI (Variables|/Game/BP/BP_PlayerRobot.BP_PlayerRobot_C|GetMGI _asbp_player_robot))))
      (bind _asumg_portal (Utilities|Casting|CastToUMG_Portal (UserInterface|GetWidget _portal_icon1)))
      (Variables|/Game/UMG/UMG_Portal.UMG_Portal_C|SetPlayer%20Index _asumg_portal 1))
    (:CastFailed
      (bind _asbp_player_samurai (Utilities|Casting|CastToBP_PlayerSamurai _returnvalue))
      (Class|WidgetComponent|SetOwnerPlayer _portal_icon1_2 (Class|Widget|GetOwningLocalPlayer (Variables|/Game/BP/BP_MainGameInstasnce.BP_MainGameInstasnce_C|GetP2%20UI (Variables|/Game/BP/BP_PlayerSamurai.BP_PlayerSamurai_C|GetMGI _asbp_player_samurai))))
      (bind _asumg_portal_2 (Utilities|Casting|CastToUMG_Portal (UserInterface|GetWidget _portal_icon1_2)))
      (Variables|/Game/UMG/UMG_Portal.UMG_Portal_C|SetPlayer%20Index _asumg_portal_2 1))))

(event EventBeginPlay
  (bind _asbp_main_game_instasnce (Utilities|Casting|CastToBP_MainGameInstasnce (Game|GetGameInstance)))
  (bind _output_get (Variables|Default|SetMGI _asbp_main_game_instasnce))
  (Variables|/Game/BP/BP_MainGameInstasnce.BP_MainGameInstasnce_C|SetWinning%20Trigger _output_get self))

(fn ConstructionScript)