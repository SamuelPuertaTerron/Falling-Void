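; Game instance for a two-player Robot and Samurai game, holding shared state across levels.
; It saves each character's items, hexes and upgrades, refunds spent skill points, then reapplies upgrades through the upgrade widgets.
; It also handles character swapping, difficulty modifiers, save loading, UI, music, enemy drops and win/lose screens.
; A backup Level 1 wave loop alternates spawns between two rows, while an external spawn manager can update the wave count.
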(event Custom|Start%20Wave
  (params (Melees :type Integer) (Spitters :type Integer))
  ;[0.3021 0.002774 0] Level 1 waves (Backup by Jake)
  (bind _output_get (Variables|Spawn|SetMelees%20To%20Spawn Melees))
  (bind _output_get_2 (Variables|Spawn|SetSpitters%20To%20Spawn Spitters))
  (Variables|Spawn|SetEnemies%20to%20Spawn (+ _output_get_2 _output_get))
  (CallFunction|WaveManager))

(event Custom|Set%20Samurai%20Stats
  (bind _samurai (Variables|Data|GetSamurai))
  ;[1 1 1] Data and Setup for new levels
  (Default|ActivateHexes _samurai (Variables|Data|GetSamurai%20Hexes))
  (Variables|/Script/FallingVoid.FVPlayerBase|SetMedkitsAmount _samurai (Utilities|Array|Get(acopy) (Variables|Data|GetMedkits%20Amount) 1))
  (Variables|/Script/FallingVoid.FVPlayerBase|SetTrapAmount _samurai (Utilities|Array|Get(acopy) (Variables|Data|GetTrap%20Amount) 1))
  (Variables|/Script/FallingVoid.FVPlayerBase|SetSkillPoints _samurai (Utilities|Array|Get(acopy) (Variables|Data|GetSkill%20Points) 1))
  (Utilities|FlowControl|Delay 0.2)
  (CallFunction|SetSamuraiUpgrades (Variables|/Game/UMG/UMG_Player1.UMG_Player1_C|GetUMG_Upgrade (Variables|/Game/BP/BP_PlayerSamurai.BP_PlayerSamurai_C|GetUI (Variables|Data|GetSamurai))) (Variables|Data|GetSamurai%20Upgrades)))

(event Custom|Spawn%20Spitter
  ;[0.3021 0.002774 0] Level 1 waves (Backup by Jake)
  (Math|Integer|IncrementInt (Variables|Spawn|GetSpitters%20Spawned)
    (:%20%20
      (Utilities|FlowControl|FlipFlop
        (:A
          (AI|SpawnAIFromClass "/Game/BP/Enemy/BP_SpitterEnemy.BP_SpitterEnemy_C" "/Game/BP/Enemy/AI/BT_MeleeEnemy.BT_MeleeEnemy" (Math|Vector|MakeVector (Variables|Spawn|GetLocation%20X%202) -3.8e+03 4.8e+02) "0, 0, 0" true 0)
          (bind _output_get (Variables|Spawn|SetLocation%20X%202 (+ (Variables|Spawn|GetLocation%20X%202) 1e+02)))
          (if (>= _output_get 5.7e+03)
            (Variables|Spawn|SetLocation%20X%202 4.7e+03)))
        (:B
          (AI|SpawnAIFromClass "/Game/BP/Enemy/BP_SpitterEnemy.BP_SpitterEnemy_C" "/Game/BP/Enemy/AI/BT_MeleeEnemy.BT_MeleeEnemy" (Math|Vector|MakeVector (Variables|Spawn|GetLocation%20X%201) -9.05e+03 3.3e+02) "0, 0, 0" true 0)
          (bind _output_get_2 (Variables|Spawn|SetLocation%20X%201 (+ (Variables|Spawn|GetLocation%20X%201) 1e+02)))
          (if (>= _output_get_2 5.7e+03)
            (Variables|Spawn|SetLocation%20X%201 4.7e+03)))))))

(event Custom|Spawn%20Melee
  ;[0.3021 0.002774 0] Level 1 waves (Backup by Jake)
  (Math|Integer|IncrementInt (Variables|Spawn|GetMelees%20Spawned)
    (:%20%20
      (Utilities|FlowControl|FlipFlop
        (:A
          (AI|SpawnAIFromClass "/Game/BP/Enemy/BP_MeleeWorking.BP_MeleeWorking_C" "/Game/BP/Enemy/AI/BT_MeleeEnemy.BT_MeleeEnemy" (Math|Vector|MakeVector (Variables|Spawn|GetLocation%20X%201) -9.05e+03 3.3e+02) "0, 0, 0" true 0)
          (bind _output_get (Variables|Spawn|SetLocation%20X%201 (+ (Variables|Spawn|GetLocation%20X%201) 1e+02)))
          (if (>= _output_get 5.7e+03)
            (Variables|Spawn|SetLocation%20X%201 4.7e+03)))
        (:B
          (AI|SpawnAIFromClass "/Game/BP/Enemy/BP_MeleeWorking.BP_MeleeWorking_C" "/Game/BP/Enemy/AI/BT_MeleeEnemy.BT_MeleeEnemy" (Math|Vector|MakeVector (Variables|Spawn|GetLocation%20X%202) -3.9e+03 4.8e+02) "0, 0, 0" true 0)
          (bind _output_get_2 (Variables|Spawn|SetLocation%20X%202 (+ (Variables|Spawn|GetLocation%20X%202) 1e+02)))
          (if (>= _output_get_2 5.7e+03)
            (Variables|Spawn|SetLocation%20X%202 4.7e+03)))))))

(event Custom|Melees
  ;[0.3021 0.002774 0] Level 1 waves (Backup by Jake)
  (if (< (- (Variables|Spawn|GetMelees%20Spawned) (Variables|Spawn|GetMelees%20Killed)) 10)
    (CallFunction|SpawnMelee)
    (CallFunction|WaveManager)))

(event Custom|SetSpawnManager
  (params (SpawnManager :type BP%20Spawn%20Manager%20Object%20Reference))
  ;[1 1 1] Sams Spawn Manager
  (bind _output_get (Variables|Ref|SetSpawnManager SpawnManager))
  (Class|FVSpawnManagerSubsystem|SetSpawnManager (Subsystems|GetFVSpawnManagerSubsystem) _output_get)
  (EventDispatchers|BindEventtoWaveChanged _output_get (delegate Custom|SetWaveCount)))

(event Custom|Target%20ending%20menu
  (bind _returnvalue (Game|GetPlayerCharacter 0))
  (bind _ending_focus (Variables|Ref|GetEnding%20focus))
  ;[1 1 1] Focus
  (Utilities|FlowControl|Delay 0.1)
  (bind _asbp_player_robot (Utilities|Casting|CastToBP_PlayerRobot _returnvalue)
    (:then
      (Default|EndingMenutoFocus _asbp_player_robot _ending_focus))
    (:CastFailed
      (bind _asbp_player_samurai (Utilities|Casting|CastToBP_PlayerSamurai _returnvalue))
      (Default|EndingMenutoFocus _asbp_player_samurai _ending_focus))))

(event Custom|Spitters
  ;[0.3021 0.002774 0] Level 1 waves (Backup by Jake)
  (if (< (- (Variables|Spawn|GetSpitters%20Spawned) (Variables|Spawn|GetSpitters%20Killed)) 2)
    (CallFunction|SpawnSpitter)
    (CallFunction|WaveManager)))

(event Custom|Add%20UI
  (bind _returnvalue (Game|GetPlayerController 0))
  ;[1 1 1] UI
  (bind _returnvalue_2 (UserInterface|CreateWidget "/Game/UMG/UMG_Main.UMG_Main_C" _returnvalue))
  (bind _output_get (Variables|UI|SetUI _returnvalue_2))
  (UserInterface|Viewport|AddtoViewport _output_get 0)
  (Input|SetInputModeGameOnly _returnvalue false)
  (Variables|/Script/Engine.PlayerController|SetbShowMouseCursor _returnvalue false)
  (bind _returnvalue_3 (UserInterface|CreateWidget "/Game/UMG/UMG_P2.UMG_P2_C" (Game|GetPlayerController 1)))
  (bind _output_get_2 (Variables|UI|SetP2%20UI _returnvalue_3))
  (UserInterface|Viewport|AddtoPlayerScreen _output_get_2))

(event Custom|Drop%20chance
  (params (Location :type Vector))
  ;[0 1 0] Enemy drops
  (if (and (Variables|Stats|GetCan%20Drop) (<= (Math|Random|RandomInteger 100) (- (Variables|Stats|GetDrop%20Rate) 1)))
    (if (Math|Random|RandomBool)
      (Game|SpawnActorfromClass "/Game/BP/Items/BP_Medkit.BP_Medkit_C" (Math|Transform|MakeTransform Location "0, 0, 0" "1.000000,1.000000,1.000000") "Undefined" "MultiplyWithRoot" 0 0)
      (else
        (Game|SpawnActorfromClass "/Game/BP/Items/BP_TrapCharger.BP_TrapCharger_C" (Math|Transform|MakeTransform Location "0, 0, 0" "1.000000,1.000000,1.000000") "Undefined" "MultiplyWithRoot" 0 0)))
    (Variables|Stats|SetCan%20Drop false)
    (Utilities|FlowControl|Delay 35.0)
    (Variables|Stats|SetCan%20Drop true)))

(event Custom|Level%20Data%20Save
  (bind _skill_points (Variables|Data|GetSkill%20Points))
  (bind _skill_points_2 (Variables|Data|GetSkill%20Points))
  ;[1 1 1] Data and Setup for new levels
  (bind _asbp_player_samurai (Utilities|Casting|CastToBP_PlayerSamurai (Game|GetPlayerCharacter (Variables|Data|GetPlayer%20To%20Swap))))
  (Variables|Data|SetSamurai _asbp_player_samurai)
  (if (== (Variables|Data|GetPlayer%20To%20Swap) 1)
    (bind _asbp_player_robot (Utilities|Casting|CastToBP_PlayerRobot (Game|GetPlayerCharacter 0)))
    (Variables|Data|SetRobot _asbp_player_robot)
    (else
      (bind _asbp_player_robot_2 (Utilities|Casting|CastToBP_PlayerRobot (Game|GetPlayerCharacter 1)))
      (Variables|Data|SetRobot _asbp_player_robot_2)))
  (Variables|Data|SetRobot%20Upgrades (Variables|/Script/FallingVoid.FVPlayerBase|GetUpgrades (Variables|Data|GetRobot)))
  (Utilities|Array|SetArrayElem (Variables|Data|GetMedkits%20Amount) 0 (Variables|/Script/FallingVoid.FVPlayerBase|GetMedkitsAmount (Variables|Data|GetRobot)))
  (Utilities|Array|SetArrayElem (Variables|Data|GetTrap%20Amount) 0 (Variables|/Script/FallingVoid.FVPlayerBase|GetTrapAmount (Variables|Data|GetRobot)))
  (Variables|Data|SetRobot%20Hexes (Variables|/Script/FallingVoid.FVPlayerBase|GetHexes (Variables|Data|GetRobot)))
  (Variables|Data|SetRobot%20Cam%20Sense (Variables|/Script/FallingVoid.FVPlayerBase|GetMouseSensitivity (Variables|Data|GetRobot)))
  (Utilities|Array|SetArrayElem (Variables|Data|GetSkill%20Points) 0 (Variables|/Script/FallingVoid.FVPlayerBase|GetSkillPoints (Variables|Data|GetRobot)))
  (bind _values (Utilities|Map|Values (Variables|Data|GetRobot%20Upgrades)))
  (for _array_element _values
    (Utilities|Array|SetArrayElem _skill_points 0 (+ (Utilities|Array|Get(acopy) _skill_points) _array_element)))
  (Variables|Data|SetSamurai%20Upgrades (Variables|/Script/FallingVoid.FVPlayerBase|GetUpgrades (Variables|Data|GetSamurai)))
  (Utilities|Array|SetArrayElem (Variables|Data|GetMedkits%20Amount) 1 (Variables|/Script/FallingVoid.FVPlayerBase|GetMedkitsAmount (Variables|Data|GetSamurai)))
  (Utilities|Array|SetArrayElem (Variables|Data|GetTrap%20Amount) 1 (Variables|/Script/FallingVoid.FVPlayerBase|GetTrapAmount (Variables|Data|GetSamurai)))
  (Variables|Data|SetSamurai%20Hexes (Variables|/Script/FallingVoid.FVPlayerBase|GetHexes (Variables|Data|GetSamurai)))
  (Utilities|Array|SetArrayElem (Variables|Data|GetSkill%20Points) 1 (Variables|/Script/FallingVoid.FVPlayerBase|GetSkillPoints (Variables|Data|GetSamurai)))
  (bind _values_2 (Utilities|Map|Values (Variables|Data|GetSamurai%20Upgrades)))
  (for _array_element_2 _values_2
    (Utilities|Array|SetArrayElem _skill_points_2 1 (+ (Utilities|Array|Get(acopy) _skill_points_2 1) _array_element_2))))

(event Custom|PlayAudioOnLevel
  (params (CurrentLevel :type E_CurrentLevel%20Enum :default "NewEnumerator0"))
  ;[1 1 1] Sams Audio
  (Variables|Default|SetCurrentLevel CurrentLevel)
  (CallFunction|UpdateCurrentAudio))

(event Custom|Level%20Set%20up
  ;[1 1 1] Data and Setup for new levels
  (Utilities|FlowControl|Delay 0.2)
  (Variables|Stats|SetRobot%20Down? false)
  (Variables|Stats|SetSamurai%20Down? false)
  (bind _asbp_player_robot (Utilities|Casting|CastToBP_PlayerRobot (Game|GetPlayerCharacter (Variables|Data|GetPlayer%20To%20Swap))))
  (Default|SwapCharacter _asbp_player_robot)
  (Widget|SetVisibility (Variables|/Game/UMG/UMG_Main.UMG_Main_C|GetUMG_CharacterSelect (Variables|UI|GetUI)) "Hidden")
  (bind _asbp_player_samurai (Utilities|Casting|CastToBP_PlayerSamurai (Game|GetPlayerCharacter (Variables|Data|GetPlayer%20To%20Swap))))
  (Variables|Data|SetSamurai _asbp_player_samurai)
  (if (== (Variables|Data|GetPlayer%20To%20Swap) 1)
    (bind _asbp_player_robot_2 (Utilities|Casting|CastToBP_PlayerRobot (Game|GetPlayerCharacter 0)))
    (Variables|Data|SetRobot _asbp_player_robot_2)
    (else
      (bind _asbp_player_robot_3 (Utilities|Casting|CastToBP_PlayerRobot (Game|GetPlayerCharacter 1)))
      (Variables|Data|SetRobot _asbp_player_robot_3)))
  (CallFunction|SetRobotStats)
  (CallFunction|SetSamuraiStats))

(event Custom|Spawn%20Enemies
  ;[0.3021 0.002774 0] Level 1 waves (Backup by Jake)
  (Utilities|FlowControl|Sequence
    (:then_0
      (if (!= (Variables|Spawn|GetMelees%20To%20Spawn) (Variables|Spawn|GetMelees%20Spawned))
        (CallFunction|Melees)))
    (:then_1
      (if (!= (Variables|Spawn|GetSpitters%20To%20Spawn) (Variables|Spawn|GetSpitters%20Spawned))
        (CallFunction|Spitters)))))

(event Custom|Wave%20Info
  (params (Melees :type Integer) (Spitters :type Integer))
  ;[0.3021 0.002774 0] Level 1 waves (Backup by Jake)
  (if (== (Variables|Spawn|GetEnemies%20killed) (Variables|Spawn|GetEnemies%20to%20Spawn))
    (if (Variables|Spawn|GetWave%20Preped)
      (CallFunction|ResetSpawns)
      (Utilities|FlowControl|Delay 3.0)
      (CallFunction|StartWave Melees Spitters)
      (else
        (Math|Integer|IncrementInt (Variables|Spawn|GetWave)
          (:%20%20
            (Variables|Spawn|SetWave%20Preped true)
            (CallFunction|WaveManager)))))
    (else
      (CallFunction|SpawnEnemies))))

(event Custom|Wave%200
  ;[0.3021 0.002774 0] Level 1 waves (Backup by Jake)
)

(event Custom|Set%20Robot%20Stats
  (bind _robot (Variables|Data|GetRobot))
  ;[1 1 1] Data and Setup for new levels
  (Default|ActivateHexes _robot (Variables|Data|GetRobot%20Hexes))
  (Variables|/Script/FallingVoid.FVPlayerBase|SetMedkitsAmount _robot (Utilities|Array|Get(acopy) (Variables|Data|GetMedkits%20Amount)))
  (Variables|/Script/FallingVoid.FVPlayerBase|SetTrapAmount _robot (Utilities|Array|Get(acopy) (Variables|Data|GetTrap%20Amount)))
  (Variables|/Script/FallingVoid.FVPlayerBase|SetSkillPoints _robot (Utilities|Array|Get(acopy) (Variables|Data|GetSkill%20Points)))
  (Variables|/Script/FallingVoid.FVPlayerBase|SetMouseSensitivity _robot (Variables|Data|GetRobot%20Cam%20Sense))
  (Utilities|FlowControl|Delay 0.2)
  (CallFunction|SetRobotUpgrades (Variables|/Game/UMG/UMG_Player1.UMG_Player1_C|GetUMG_Upgrade (Variables|/Game/BP/BP_PlayerRobot.BP_PlayerRobot_C|GetUI (Variables|Data|GetRobot))) (Variables|Data|GetRobot%20Upgrades)))

(event Custom|UpdateCurrentAudio
  ;[1 1 1] Sams Audio
  (Utilities|FlowControl|Delay 0.2)
  (switch Utilities|FlowControl|Switch|SwitchonE_CurrentLevel (Variables|Default|GetCurrentLevel)
    (:NewEnumerator0
      (Audio|PlaySound2D "/Game/Sounds/Music/Sound_MusicLevel1.Sound_MusicLevel1" 1.0 1.0 0.0 "/Game/Sounds/Con_Music.Con_Music" 0))
    (:NewEnumerator1
      (Audio|PlaySound2D "/Game/Sounds/Music/Sound_MusicLevel2.Sound_MusicLevel2" 1.0 1.0 0.0 "/Game/Sounds/Con_Music.Con_Music" 0))
    (:NewEnumerator2
      (Audio|PlaySound2D "/Game/Sounds/Music/Sound_MusicBoss.Sound_MusicBoss" 1.0 1.0 0.0 "/Game/Sounds/Con_Music.Con_Music" 0))
    (:NewEnumerator3
      (Audio|PlaySound2D "/Game/Sounds/Music/Sound_MusicCompleted.Sound_MusicCompleted" 1.0 1.0 0.0 "/Game/Sounds/Con_Music.Con_Music" 0))
    (:NewEnumerator4
      (Audio|PlaySound2D "/Game/Sounds/Music/Sound_MusicFailed.Sound_MusicFailed" 1.0 1.0 0.0 "/Game/Sounds/Con_Music.Con_Music" 0))
    (:NewEnumerator5
      (Audio|PlaySound2D "/Game/Sounds/Music/Sound_MusicCharacterSelect.Sound_MusicCharacterSelect" 1.0 1.0 0.0 "/Game/Sounds/Con_Music.Con_Music" 0))
    (:NewEnumerator6
      (Audio|PlaySound2D "/Game/Sounds/Music/Sound_MusicGeneral.Sound_MusicGeneral" 1.0 1.0 0.0 "/Game/Sounds/Con_Music.Con_Music" 0))))

(event Custom|SetBoss
  (params (Boss :type BP%20Boss%20Object%20Reference))
  ;[1 1 1] Sams Audio
  (Variables|Ref|SetBoss Boss))

(event Custom|SetWaveCount
  (params (Wave :type Integer))
  ;[1 1 1] Sams Spawn Manager
  (Variables|Spawn|SetWave Wave))

(event Custom|Winning
  (bind _returnvalue (Game|GetPlayerController 0))
  (bind _ui (Variables|UI|GetUI))
  (bind _umg_level1complete (Variables|/Game/UMG/UMG_Main.UMG_Main_C|GetUMG_Level1Complete _ui))
  ;[1 1 1] Endings
  (Variables|Stats|SetLevel%20Ending true)
  (Variables|Stats|SetRobot%20Down? false)
  (Variables|Stats|SetSamurai%20Down? false)
  (Utilities|Time|SetGlobalTimeDilation 0.1)
  (Widget|SetVisibility _umg_level1complete "Visible")
  (UserInterface|Animation|PlayAnimation _umg_level1complete (Variables|/Game/UMG/UMG_LevelComplete.UMG_LevelComplete_C|GetBlackoutFade _umg_level1complete) 0.0 1 "Forward" 1.0 false)
  (Utilities|FlowControl|Delay 0.5)
  (Widget|SetVisibility (Variables|/Game/UMG/UMG_LevelComplete.UMG_LevelComplete_C|GetWinningBorder _umg_level1complete) "Visible")
  (if (!= (Variables|Data|GetLevel) 3)
    (Variables|Ref|SetEnding%20focus (Variables|/Game/UMG/UMG_LevelComplete.UMG_LevelComplete_C|GetNextLevel _umg_level1complete))
    (else
      (Variables|Ref|SetEnding%20focus (Variables|/Game/UMG/UMG_LevelComplete.UMG_LevelComplete_C|GetMenu _umg_level1complete))))
  (Utilities|Time|SetGlobalTimeDilation 1.0)
  (Input|SetInputModeGameandUI _returnvalue _umg_level1complete "DoNotLock" true false)
  (Variables|/Script/Engine.PlayerController|SetbShowMouseCursor _returnvalue true)
  (Input|SetInputModeGameandUI (Game|GetPlayerController 1) _umg_level1complete "DoNotLock" true false)
  (CallFunction|TargetEndingMenu))

(event Custom|Diffculty%20Mods
  ;[0 0.1767 1] Diffculty
  (switch int (Variables|Diffculty|GetDiffculty)
    (:1
      (Variables|Diffculty|SetEnemy%20Dmg%20Boost 0.8)
      (Variables|Diffculty|SetEnemy%20Health%20Mod 0.5)
      (Variables|Diffculty|SetEnemy%20speed%20Mod 0.8)
      (Variables|Diffculty|SetLives 5))
    (:2
      (Variables|Diffculty|SetEnemy%20Dmg%20Boost 1.0)
      (Variables|Diffculty|SetEnemy%20Health%20Mod 1.0)
      (Variables|Diffculty|SetEnemy%20speed%20Mod 1.0)
      (Variables|Diffculty|SetLives 3))
    (:3
      (Variables|Diffculty|SetEnemy%20Dmg%20Boost 1.2)
      (Variables|Diffculty|SetEnemy%20Health%20Mod 1.5)
      (Variables|Diffculty|SetEnemy%20speed%20Mod 1.2)
      (Variables|Diffculty|SetLives 1))
    (:4
      (Variables|Diffculty|SetEnemy%20Dmg%20Boost 5.0)
      (Variables|Diffculty|SetEnemy%20Health%20Mod 2.0)
      (Variables|Diffculty|SetEnemy%20speed%20Mod 1.5)
      (Variables|Diffculty|SetLives 0))))

(event Custom|SwapCharacter
  (params (Transform :type Transform) (Target :type Actor%20Object%20Reference))
  (bind _player_to_swap (Variables|Data|GetPlayer%20To%20Swap))
  ;[1 1 1] Swap character
  (bind _output_get (Variables|Stats|SetTransform Transform))
  (Actor|DestroyActor Target)
  (bind _returnvalue (Game|SpawnActorfromClass "/Game/BP/BP_PlayerSamurai.BP_PlayerSamurai_C" _output_get "Undefined" "MultiplyWithRoot" 0 0))
  (Pawn|Possess (Game|GetPlayerController _player_to_swap) _returnvalue)
  (Variables|/Game/BP/BP_PlayerSamurai.BP_PlayerSamurai_C|SetMGI _returnvalue self)
  (if (== _player_to_swap 1)
    (Variables|/Game/BP/BP_PlayerSamurai.BP_PlayerSamurai_C|SetPlayer1? _returnvalue false)
    (bind _asbp_player_robot (Utilities|Casting|CastToBP_PlayerRobot (Game|GetPlayerCharacter 0)))
    (Variables|/Game/BP/BP_PlayerRobot.BP_PlayerRobot_C|SetPlayer1? _asbp_player_robot true)
    (Default|UISet _asbp_player_robot)
    (else
      (Variables|/Game/BP/BP_PlayerSamurai.BP_PlayerSamurai_C|SetPlayer1? _returnvalue true)
      (bind _asbp_player_robot_2 (Utilities|Casting|CastToBP_PlayerRobot (Game|GetPlayerCharacter 1))
        (:then
          (Variables|/Game/BP/BP_PlayerRobot.BP_PlayerRobot_C|SetPlayer1? _asbp_player_robot_2 false)
          (Default|UISet _asbp_player_robot_2))
        (:CastFailed
          _))))
  (Transformation|Teleport _returnvalue (Variables|Stats|GetHikari%20SpawnPoint) (Variables|Stats|GetKikari%20Dest%20Rotation))
  (Default|UISet _returnvalue))

(event Custom|Check%20for%20losing
  (bind _returnvalue (Game|GetPlayerController 0))
  (bind _ui (Variables|UI|GetUI))
  (bind _umg_gameover (Variables|/Game/UMG/UMG_Main.UMG_Main_C|GetUMG_GameOver _ui))
  ;[1 1 1] Endings
  (if (and (Variables|Stats|GetRobot%20Down?) (Variables|Stats|GetSamurai%20Down?))
    (Variables|Stats|SetLevel%20Ending true)
    (Variables|Stats|SetRobot%20Down? false)
    (Variables|Stats|SetSamurai%20Down? false)
    (Utilities|Time|SetGlobalTimeDilation 0.1)
    (Widget|SetVisibility _umg_gameover "Visible")
    (UserInterface|Animation|PlayAnimation _umg_gameover (Variables|/Game/UMG/UMG_GameOver.UMG_GameOver_C|GetBlackoutFade _umg_gameover) 0.0 1 "Forward" 1.0 false)
    (Utilities|FlowControl|Delay 0.5)
    (Widget|SetVisibility (Variables|/Game/UMG/UMG_GameOver.UMG_GameOver_C|GetLoserBorder _umg_gameover) "Visible")
    (Variables|Ref|SetEnding%20focus (Variables|/Game/UMG/UMG_GameOver.UMG_GameOver_C|GetRetry _umg_gameover))
    (Utilities|Time|SetGlobalTimeDilation 1.0)
    (Input|SetInputModeGameandUI _returnvalue _umg_gameover "DoNotLock" true false)
    (Variables|/Script/Engine.PlayerController|SetbShowMouseCursor _returnvalue true)
    (Input|SetInputModeGameandUI (Game|GetPlayerController 1) _umg_gameover "DoNotLock" true false)
    (CallFunction|TargetEndingMenu)))

(event Custom|Wave%20Manager
  ;[0.3021 0.002774 0] Level 1 waves (Backup by Jake)
  (switch int (Variables|Spawn|GetWave)
    (:0
      (CallFunction|WaveInfo 2))
    (:1
      (CallFunction|WaveInfo 2 2))
    (:2
      (CallFunction|WaveInfo 5 3))
    (:3
      (CallFunction|WaveInfo 10 5))
    (:4
      (CallFunction|WaveInfo 15 7))
    (:5
      (Variables|Spawn|SetWave 0)
      (CallFunction|Winning))))

(event Custom|Reset%20spawns
  ;[0.3021 0.002774 0] Level 1 waves (Backup by Jake)
  (Variables|Spawn|SetMelees%20Spawned 0)
  (Variables|Spawn|SetSpitters%20Spawned 0)
  (Variables|Spawn|SetEnemies%20killed 0)
  (Variables|Spawn|SetSpitters%20Killed 0)
  (Variables|Spawn|SetMelees%20Killed 0)
  (Variables|Spawn|SetWave%20Preped false))

(event EventInit
  ;[1 1 1] Save Game
  (bind _returnvalue (SaveGame|DoesSaveGameExist "1"))
  (if _returnvalue
    (bind _returnvalue_2 (SaveGame|LoadGamefromSlot (Variables|Ref|GetSaveSlot)))
    (bind _asbp_save_game_instance (Utilities|Casting|CastToBP_SaveGameInstance _returnvalue_2))
    (Variables|Ref|SetSGI _asbp_save_game_instance)
    (else
      (bind _returnvalue_3 (SaveGame|CreateSaveGameObject "/Game/BP/BP_SaveGameInstance.BP_SaveGameInstance_C"))
      (bind _output_get (Variables|Ref|SetSGI _returnvalue_3))
      (SaveGame|SaveGametoSlot _output_get (Variables|Ref|GetSaveSlot)))))

(fn SetEnemyDiffculty
  (params (Enemy :type FV%20Enemy%20Base%20Object%20Reference))
  (bind _output_get (Variables|/Script/FallingVoid.FVBaseCharacter|SetMaxHealth Enemy (* (Variables|/Script/FallingVoid.FVBaseCharacter|GetHealth Enemy) (Variables|Diffculty|GetEnemy%20Health%20Mod))))
  (Variables|/Script/FallingVoid.FVBaseCharacter|SetHealth Enemy _output_get)
  (Variables|/Script/FallingVoid.FVBaseCharacter|SetDamageBoost Enemy (Variables|Diffculty|GetEnemy%20Dmg%20Boost))
  (Variables|/Script/Engine.CharacterMovementComponent|SetMaxWalkSpeed (Variables|/Script/Engine.Character|GetCharacterMovement Enemy) (* (Variables|Diffculty|GetEnemy%20speed%20Mod) (Variables|/Script/FallingVoid.FVEnemyBase|GetSpeedModifer Enemy))))

(fn SetRobotUpgrades
  (params (Upgrade%20UI :type UMG%20Upgrade%20Object%20Reference) (Upgrades :type Map%20of%20Strings%20to%20Integers))
  (bind _rhealthbutton2 (Variables|/Game/UMG/UMG_Upgrade.UMG_Upgrade_C|GetRHealthButton2 Upgrade%20UI))
  (bind _rweaponbutton2 (Variables|/Game/UMG/UMG_Upgrade.UMG_Upgrade_C|GetRWeaponButton2 Upgrade%20UI))
  (bind _ra1button2 (Variables|/Game/UMG/UMG_Upgrade.UMG_Upgrade_C|GetRA1Button2 Upgrade%20UI))
  (bind _ra2button2 (Variables|/Game/UMG/UMG_Upgrade.UMG_Upgrade_C|GetRA2Button2 Upgrade%20UI))
  (bind _ra3button2 (Variables|/Game/UMG/UMG_Upgrade.UMG_Upgrade_C|GetRA3Button2 Upgrade%20UI))
  (bind _rmedkitbutton2 (Variables|/Game/UMG/UMG_Upgrade.UMG_Upgrade_C|GetRMedkitButton2 Upgrade%20UI))
  (bind _values (Utilities|Map|Values Upgrades))
  (for (_array_element _array_index) _values
    (if (!= _array_element 0)
      (switch int _array_index
        (:0
          (Default|RUpgradeHealth Upgrade%20UI 1.2 1 (Variables|/Game/UMG/UMG_Upgrade.UMG_Upgrade_C|GetRHealthButton1 Upgrade%20UI) _rhealthbutton2)
          (if (== _array_element 2)
            (Default|RUpgradeHealth Upgrade%20UI 1.25 2 _rhealthbutton2)))
        (:1
          (Default|RUpgradeMedkit Upgrade%20UI 1.5 (Variables|/Game/UMG/UMG_Upgrade.UMG_Upgrade_C|GetRMedkitButton1 Upgrade%20UI) _rmedkitbutton2)
          (if (== _array_element 2)
            (Default|RUpgradeMedkit Upgrade%20UI 1.5 _rmedkitbutton2)))
        (:2
          (Default|RUpgradeWeapon Upgrade%20UI 1.0 (Variables|/Game/UMG/UMG_Upgrade.UMG_Upgrade_C|GetRWeaponButton1 Upgrade%20UI) _rweaponbutton2 5.0)
          (if (== _array_element 2)
            (Default|RUpgradeWeapon Upgrade%20UI 1.0 _rweaponbutton2 0 5.0)))
        (:3
          (Default|RUpgradeA1 Upgrade%20UI 1.5 (Variables|/Game/UMG/UMG_Upgrade.UMG_Upgrade_C|GetRA1Button1 Upgrade%20UI) _ra1button2 1.2)
          (if (== _array_element 2)
            (Default|RUpgradeA1 Upgrade%20UI 1.5 _ra1button2 0 1.2)))
        (:4
          (Default|RUpgradeA2 Upgrade%20UI 1.5 (Variables|/Game/UMG/UMG_Upgrade.UMG_Upgrade_C|GetRA2Button1 Upgrade%20UI) _ra2button2 1.3)
          (if (== _array_element 2)
            (Default|RUpgradeA2 Upgrade%20UI 1.5 _ra2button2 0 1.3)))
        (:5
          (Default|RUpgradeA3 Upgrade%20UI (Variables|/Game/UMG/UMG_Upgrade.UMG_Upgrade_C|GetRA3Button1 Upgrade%20UI) _ra3button2)
          (if (== _array_element 2)
            (Default|RUpgradeA3 Upgrade%20UI _ra3button2))))))
  (return))

(fn SetSamuraiUpgrades
  (params (Upgrade%20UI :type UMG%20Upgrade%20Object%20Reference) (Upgrades :type Map%20of%20Strings%20to%20Integers))
  (bind _sa2button2 (Variables|/Game/UMG/UMG_Upgrade.UMG_Upgrade_C|GetSA2Button2 Upgrade%20UI))
  (bind _subutton2 (Variables|/Game/UMG/UMG_Upgrade.UMG_Upgrade_C|GetSUButton2 Upgrade%20UI))
  (bind _sa1button2 (Variables|/Game/UMG/UMG_Upgrade.UMG_Upgrade_C|GetSA1Button2 Upgrade%20UI))
  (bind _shealthbutton2 (Variables|/Game/UMG/UMG_Upgrade.UMG_Upgrade_C|GetSHealthButton2 Upgrade%20UI))
  (bind _smedkitbutton2 (Variables|/Game/UMG/UMG_Upgrade.UMG_Upgrade_C|GetSMedkitButton2 Upgrade%20UI))
  (bind _sweaponbutton2 (Variables|/Game/UMG/UMG_Upgrade.UMG_Upgrade_C|GetSWeaponButton2 Upgrade%20UI))
  (bind _values (Utilities|Map|Values Upgrades))
  (for (_array_element _array_index) _values
    (if (!= _array_element 0)
      (switch int _array_index
        (:0
          (Default|SUpgradeHealth Upgrade%20UI 1.2 0 (Variables|/Game/UMG/UMG_Upgrade.UMG_Upgrade_C|GetSHealthButton1 Upgrade%20UI) _shealthbutton2)
          (if (== _array_element 2)
            (Default|SUpgradeHealth Upgrade%20UI 1.25 0 _shealthbutton2)))
        (:1
          (Default|SUpgradeMedkit Upgrade%20UI 1.5 (Variables|/Game/UMG/UMG_Upgrade.UMG_Upgrade_C|GetSMedkitButton1 Upgrade%20UI) _smedkitbutton2)
          (if (== _array_element 2)
            (Default|SUpgradeMedkit Upgrade%20UI 1.5 _smedkitbutton2)))
        (:2
          (Default|SUpgradeWeapon Upgrade%20UI 4.0 (Variables|/Game/UMG/UMG_Upgrade.UMG_Upgrade_C|GetSWeaponButton1 Upgrade%20UI) _sweaponbutton2 2e+01)
          (if (== _array_element 2)
            (Default|SUpgradeWeapon Upgrade%20UI 4.0 _sweaponbutton2 0 2e+01)))
        (:3
          (Default|SUpgradeA1 Upgrade%20UI 1.5 25.0 (Variables|/Game/UMG/UMG_Upgrade.UMG_Upgrade_C|GetSA1Button1 Upgrade%20UI) _sa1button2)
          (if (== _array_element 2)
            (Default|SUpgradeA1 Upgrade%20UI 1.5 25.0 _sa1button2)))
        (:4
          (Default|SUpgradeA2 Upgrade%20UI 35.0 (Variables|/Game/UMG/UMG_Upgrade.UMG_Upgrade_C|GetSA2Button1 Upgrade%20UI) _sa2button2)
          (if (== _array_element 2)
            (Default|SUpgradeA2 Upgrade%20UI 35.0 _sa2button2)))
        (:5
          (Default|SUpgradeUtility Upgrade%20UI 1e+02 (Variables|/Game/UMG/UMG_Upgrade.UMG_Upgrade_C|GetSUButton1 Upgrade%20UI) _subutton2)
          (if (== _array_element 2)
            (Default|SUpgradeUtility Upgrade%20UI 1e+02 _subutton2))))))
  (return))